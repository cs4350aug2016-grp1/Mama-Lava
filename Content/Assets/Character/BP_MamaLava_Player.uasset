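; BP_MamaLava_Player is the player character, with movement along world X only, plus jump and hold-to-crouch.
; On BeginPlay it enables camera pawn-control rotation only if a head-mounted display is active, then detaches the camera root from the capsule.
; Each Tick moves the camera root to the capsule's world location, so the camera follows position without inheriting the capsule's rotation.
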(event `InputAxis|Move Right`
  (params (AxisValue :type "Float (single-precision)"))
  (`self.AddMovementInput` (1.0 0.0 0.0) AxisValue))

(event `self.ReceiveBeginPlay`
  (set `CameraComponent.bUsePawnControlRotation` (`HeadMountedDisplayFunctionLibrary.IsHeadMountedDisplayEnabled`) (`self.Camera`))
  (`SceneComponent.K2_DetachFromComponent` (`self.CameraRoot`) "KeepWorld" "KeepRelative" "KeepRelative" true))

(event `self.ReceiveTick`
  (params (DeltaSeconds :type "Float (single-precision)"))
  (`SceneComponent.K2_SetWorldLocation` (`self.CameraRoot`) (`SceneComponent.K2_GetComponentLocation` (`self.CapsuleComponent`)) false false))

(event `InputAction|Jump`
  (params (Key :type "Key Structure" :default "AnyKey"))
  (:`Pressed`
    (`self.Jump`)))

(event `InputAction|Duck`
  (params (Key :type "Key Structure" :default "AnyKey"))
  (:`Pressed`
    (`self.Crouch`))
  (:`Released`
    (`self.UnCrouch`)))

(fn `UserConstructionScript`)