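; Tooltip activator for the magnet character, which triggers a tooltip when a BP_Magnet enters its collision sphere.
; On overlap it casts the other actor to BP_Magnet and passes the result of GetRandomTooltip to that magnet's ShowTooltip.
; The Get Random Tooltip graph holds a random pick from the Tooltips array, but that node is unused.
; Construction only calls the parent script.
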(event `self.CollisionSphere.OnComponentBeginOverlap`
  (params (OverlappedComponent :type "PrimitiveComponent Object Reference") (OtherActor :type "Actor Object Reference") (OtherComp :type "PrimitiveComponent Object Reference") (OtherBodyIndex :type Integer) (bFromSweep :type Boolean) (SweepResult :type "HitResult Structure (by ref)"))
  (bind _asbp_magnet (cast `/Game/Blueprints/Environment/Pickup/BP_Magnet` OtherActor))
  ;[1 1 1] Show tooltip with text and effect
  (`/Game/Blueprints/Environment/Pickup/BP_Pickup.Show Tooltip` _asbp_magnet (`KismetArrayLibrary.Array_Get` (`self.Tooltips`) (`KismetMathLibrary.RandomIntegerInRange` 0 (- (`KismetArrayLibrary.Array_Length` (`self.Tooltips`)) 1)))))

(fn `UserConstructionScript`
  (`parent.UserConstructionScript`))