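; Tooltip trigger that makes pickups of an assigned class display a tooltip when they enter its collision sphere.
; On overlap, it requires an exact PickUpClass match, casts the actor to BP_Pickup and passes GetRandomTooltip's result to ShowTooltip.
; The Get Random Tooltip graph contains a random-index lookup into the Tooltips array, though that lookup is left unconnected.
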(event `self.CollisionSphere.OnComponentBeginOverlap`
  (params (OverlappedComponent :type "PrimitiveComponent Object Reference") (OtherActor :type "Actor Object Reference") (OtherComp :type "PrimitiveComponent Object Reference") (OtherBodyIndex :type Integer) (bFromSweep :type Boolean) (SweepResult :type "HitResult Structure (by ref)"))
  ;[1 1 1] Check only the assigned PickUpClass
  (if (== (`GameplayStatics.GetObjectClass` OtherActor) (`self.PickUpClass`))
    (bind _asbp_pickup (cast `/Game/Blueprints/Environment/Pickup/BP_Pickup` OtherActor))
    ;[1 1 1] Show tooltip with text and effect
    (`/Game/Blueprints/Environment/Pickup/BP_Pickup.Show Tooltip` _asbp_pickup (`KismetArrayLibrary.Array_Get` (`self.Tooltips`) (`KismetMathLibrary.RandomIntegerInRange` 0 (- (`KismetArrayLibrary.Array_Length` (`self.Tooltips`)) 1))))))

(fn `UserConstructionScript`)