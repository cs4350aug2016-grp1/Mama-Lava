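; Tooltip activator actor that triggers tooltips on AntiCoins that overlap its collision sphere.
; Each overlap with a BP_AntiCoin passes the result of GetRandomTooltip to that coin's ShowTooltip and increments an encounter counter.
; The activator destroys itself once the count exceeds MaxEncounterCount.
; In GetRandomTooltip, the random pick from the Tooltips array is present but left unused.
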(event `self.CollisionSphere.OnComponentBeginOverlap`
  (params (OverlappedComponent :type "PrimitiveComponent Object Reference") (OtherActor :type "Actor Object Reference") (OtherComp :type "PrimitiveComponent Object Reference") (OtherBodyIndex :type Integer) (bFromSweep :type Boolean) (SweepResult :type "HitResult Structure (by ref)"))
  (bind _asbp_anti_coin (cast `/Game/Blueprints/Environment/Pickup/BP_AntiCoin` OtherActor))
  ;[1 1 1] Show tooltip with text and effect
  (`/Game/Blueprints/Environment/Pickup/BP_Pickup.Show Tooltip` _asbp_anti_coin (`KismetArrayLibrary.Array_Get` (`self.Tooltips`) (`KismetMathLibrary.RandomIntegerInRange` 0 (- (`KismetArrayLibrary.Array_Length` (`self.Tooltips`)) 1))))
  ;[1 1 1] Destroy actor when encounter AntiCoins the max encouter count
  (bind _result (`/Engine/EditorBlueprintResources/StandardMacros.IncrementInt` (`self.EncouterCount`))
    (:`  `
      (if (> _result (`self.MaxEncounterCount`))
        (`self.K2_DestroyActor`)))))

(fn `UserConstructionScript`
  (`parent.UserConstructionScript`))