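; Player character for MamaLava with VR support, camera-relative movement, jumping and an optional double jump.
; On begin play it detaches the camera and instruction text; each tick the camera eases to capsule height and turns toward the player, while the text floats overhead facing the camera.
; Left/right input also advances a looping-aware spline distance, but the spline-snapping logic is never run.
; Helper functions spawn pickups and tooltip activators and hide instructions by score.
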(event EventBeginPlay
  ;[1 1 1] Begin Play
  (|EnableCameraRotationforHMD)
  (|DetachCameraFromCapsule)
  (|DetachInstructionTextFromCapsule))

(event EventTick
  (params (DeltaSeconds :type Float%20%28single-precision%29))
  ;[1 1 1] Per Frame Operations
  (|SetCameratoCurrentHeightofCapsule)
  (|RotateCameratoPointatPlayer)
  (|RotateandLocateInstructionTexttoPointatCamera))

(event EventOnLanded
  (params (Hit :type Hit%20Result%20Structure%20%28by%20ref%29))
  ;[1 1 1] Movement Related
  (Utilities|FlowControl|DoN 2) ; enters at Reset
)

(event Input|ActionEvents|InputActionJump
  (params (Key :type Key%20Structure :default "AnyKey"))
  ;[1 1 1] Movement Related
  (:Pressed
    (if (Variables|Default|GetCanDoubleJump)
      (bind _counter (Utilities|FlowControl|DoN 2)
        (:Exit
          (switch int _counter
            (:1
              (Character|Jump))
            (:2
              (Character|LaunchCharacter (Math|Vector|MakeVector 0.0 0.0 (Variables|/Script/Engine.CharacterMovementComponent|GetJumpZVelocity (Variables|Character|GetCharacterMovement))) false true)))))
      (elif (AI|Components|NavMovement|IsMovingonGround (Variables|Character|GetCharacterMovement))
        (Audio|PlaySoundatLocation "/Game/Assets/StarterContent/Audio/jump_Cue.Jump_Cue" "0, 0, 0")
        (Character|Jump)))))

(event Input|ActionEvents|InputActionResetVR
  (params (Key :type Key%20Structure :default "AnyKey"))
  ;[1 1 1] Movement Related
  (:Pressed
    (Class|HeadMountedDisplayFunctionLibrary|ResetOrientationandPosition 0.0 "OrientationAndPosition")))

(event Input|ActionEvents|InputActionDebugToggleMouse
  (params (Key :type Key%20Structure :default "AnyKey"))
  (bind _camera (Variables|Default|GetCamera))
  ;[1 1 1] Mouse input: Debug
  (:Pressed
    (Variables|/Script/Engine.CameraComponent|SetbUsePawnControlRotation _camera (not (Variables|/Script/Engine.CameraComponent|GetbUsePawnControlRotation _camera)))))

(event Input|AxisEvents|InputAxisMoveLeft
  (params (AxisValue :type Float%20%28single-precision%29))
  ;[1 1 1] Movement Related
  (Utilities|IsThereACurrentSplinetoFollow
    (:Yes
      (|AlterInterpolatedSplineValue AxisValue))
    (:No
      _))
  (|ExecuteLeftRightRun AxisValue))

(event Input|AxisEvents|InputAxisLookUp
  (params (AxisValue :type Float%20%28single-precision%29))
  ;[1 1 1] Mouse input: Debug
  (Pawn|Input|AddControllerPitchInput AxisValue))

(event Input|AxisEvents|InputAxisTurn
  (params (AxisValue :type Float%20%28single-precision%29))
  ;[1 1 1] Mouse input: Debug
  (Pawn|Input|AddControllerYawInput AxisValue))

(event Input|AxisEvents|InputAxisMoveForward
  (params (AxisValue :type Float%20%28single-precision%29))
  ;[1 1 1] Movement Related
  (Utilities|IsThereACurrentSplinetoFollow
    (:Yes
      _)
    (:No
      _))
  (|ExecuteForwardBackwardsRun AxisValue))

(fn ConstructionScript
  (bind _charactermovement (Variables|Character|GetCharacterMovement))
  ;[1 1 1] Save base stats
  (Variables|BaseStats|SetBaseJumpingZVelocity (Variables|/Script/Engine.CharacterMovementComponent|GetJumpZVelocity _charactermovement))
  (Variables|BaseStats|SetBaseMaxWalkSpeed (Variables|/Script/Engine.CharacterMovementComponent|GetMaxWalkSpeed _charactermovement)))

(fn OutputDistanceAlongSpline
  (params (Spline :type BP%20Spline%20Single%20Mesh%20Platform%20Old%20Object%20Reference) (Number_Of_Samples :type Float%20%28single-precision%29))
  (LocalVariables|SetSuppliedSpline (Variables|/Game/Blueprints/Environment/Spline/Old/BP_Spline_Single_Mesh_Platform_Old.BP_Spline_Single_Mesh_Platform_Old_C|GetSpline Spline))
  (LocalVariables|SetNumberOfSamples Number_Of_Samples)
  (LocalVariables|SetLocationAlongSpline (|CalculateClosestDistanceonSplinetoCurrentLocation))
  (while (< (LocalVariables|GetRecordedDistanceAlongSpline) (Spline|GetSplineLength (LocalVariables|GetSuppliedSpline)))
    (if (< (Math|Float|Sqrt (Math|Float|Square (Math|Vector|DotProduct (- (Spline|GetLocationatDistanceAlongSpline (LocalVariables|GetSuppliedSpline) (LocalVariables|GetRecordedDistanceAlongSpline) "World") (LocalVariables|GetLocationAlongSpline)) (- (Spline|GetLocationatDistanceAlongSpline (LocalVariables|GetSuppliedSpline) (LocalVariables|GetRecordedDistanceAlongSpline) "World") (LocalVariables|GetLocationAlongSpline))))) (LocalVariables|GetLowestDisplacementThusFar))
      (LocalVariables|SetLowestDisplacementThusFar (Math|Float|Sqrt (Math|Float|Square (Math|Vector|DotProduct (- (Spline|GetLocationatDistanceAlongSpline (LocalVariables|GetSuppliedSpline) (LocalVariables|GetRecordedDistanceAlongSpline) "World") (LocalVariables|GetLocationAlongSpline)) (- (Spline|GetLocationatDistanceAlongSpline (LocalVariables|GetSuppliedSpline) (LocalVariables|GetRecordedDistanceAlongSpline) "World") (LocalVariables|GetLocationAlongSpline))))))
      (LocalVariables|SetDistanceWhichHasLowestDisplacementThusFar (LocalVariables|GetRecordedDistanceAlongSpline)))
    (|IncrementRecordedDistanceAlongSpline))
  (return (LocalVariables|GetDistanceWhichHasLowestDisplacementThusFar) (Spline|GetLocationatDistanceAlongSpline (LocalVariables|GetSuppliedSpline) (LocalVariables|GetDistanceWhichHasLowestDisplacementThusFar) "World")))

(fn InstructionVisibility
  (if (not (< (Variables|Default|GetScore) 2e+02))
    (Rendering|SetVisibility (Variables|Default|GetInstructionText) false false)))

(fn AddTooltipActivator
  (params (TooltipActivatorClass :type BP%20Tooltip%20Activator%20Class%20Reference))
  ;[1 1 1] Spawn the Tooltip Activator of the given class
  (bind _returnvalue (Game|SpawnActorfromClass TooltipActivatorClass (Transformation|GetActorTransform) "Undefined" self 0))
  (bind _output_get (LocalVariables|SetTooltipActivator _returnvalue))
  ;[1 1 1] Add Tooltip to an array to keep track of it when deleting
  (Utilities|IsValid _output_get
    (:Is%20Valid
      (Transformation|AttachActorToActor (LocalVariables|GetTooltipActivator) self "None" "KeepWorld" "KeepWorld" "KeepWorld" true)
      (Utilities|Array|Add (Variables|Tooltips|GetTooltipActivators) (LocalVariables|GetTooltipActivator)))))

(fn SpawnPickUpinFront
  (params (PickUpClass :type BP%20Pickup%20Class%20Reference))
  (Game|SpawnActorfromClass PickUpClass (Math|Conversions|ToTransform(Vector) (+ (.location (Transformation|GetActorTransform)) (* (Transformation|GetActorForwardVector) 1.2e+02))) "Undefined" 0 0))