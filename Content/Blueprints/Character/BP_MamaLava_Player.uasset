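; Player character for a VR-capable climbing platformer that runs along spline platforms and scores points for each new best height.
; Overlapping a platform spline snaps it to the nearest sampled distance; left/right input moves that distance, wrapping on closed loops, and jumping detaches.
; A detached camera tracks capsule height and turns toward the player, as floating score and instruction text face the camera.
; Also handles platform pass-through, tooltip activators and debug inputs.
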(event OnComponentBeginOverlap(SplineTriggerArea)
  (params (OverlappedComponent :type Primitive%20Component%20Object%20Reference) (OtherActor :type Actor%20Object%20Reference) (OtherComp :type Primitive%20Component%20Object%20Reference) (OtherBodyIndex :type Integer) (bFromSweep :type Boolean) (SweepResult :type Hit%20Result%20Structure%20%28by%20ref%29))
  ;[1 1 1] Spline Replated Functionality
  (|CastAndAttachToSplineIfPossible OtherComp))

(event OnComponentBeginOverlap(PlatformCollisionBuffer)
  (params (OverlappedComponent :type Primitive%20Component%20Object%20Reference) (OtherActor :type Actor%20Object%20Reference) (OtherComp :type Primitive%20Component%20Object%20Reference) (OtherBodyIndex :type Integer) (bFromSweep :type Boolean) (SweepResult :type Hit%20Result%20Structure%20%28by%20ref%29))
  ;[1 1 1] Platform Collision Functionality
  (bind _asbp_spline_single_mesh_platform (Utilities|Casting|CastToBP_Spline_Single_Mesh_Platform OtherActor))
  (Collision|IgnoreActorwhenMoving (Variables|Collision|GetCapsuleComponent) _asbp_spline_single_mesh_platform true))

(event OnComponentEndOverlap(PlatformCollisionBuffer)
  (params (OverlappedComponent :type Primitive%20Component%20Object%20Reference) (OtherActor :type Actor%20Object%20Reference) (OtherComp :type Primitive%20Component%20Object%20Reference) (OtherBodyIndex :type Integer))
  ;[1 1 1] Platform Collision Functionality
  (bind _asbp_spline_single_mesh_platform (Utilities|Casting|CastToBP_Spline_Single_Mesh_Platform OtherActor))
  (Collision|IgnoreActorwhenMoving (Variables|Collision|GetCapsuleComponent) _asbp_spline_single_mesh_platform false))

(event Custom|Attach%20To%20Spline
  (params (Spine :type BP%20Spline%20Single%20Mesh%20Platform%20Object%20Reference))
  ;[1 1 1] Spline Replated Functionality
  (|SetupSpline Spine))

(event Custom|DisableCoinTooltip
  (bind _coinstooltipactivator (Variables|Tooltips|GetCoinsTooltipActivator))
  ;[1 1 1] Disable tooltips events
  (Utilities|FlowControl|DoOnce false
    (:Completed
      (if (Utilities|IsValid _coinstooltipactivator)
        (Actor|DestroyActor _coinstooltipactivator)))))

(event Custom|Detach%20From%20Spline
  ;[1 1 1] Spline Replated Functionality
  (Variables|Default|SetIsThereAnActiveSpline false)
  (|TemporarilyDisableCollisionSphere))

(event Custom|DisableMagnetTooltip
  (bind _magnetstooltipactivator (Variables|Tooltips|GetMagnetsTooltipActivator))
  ;[1 1 1] Disable tooltips events
  (Utilities|FlowControl|DoOnce false
    (:Completed
      (if (Utilities|IsValid _magnetstooltipactivator)
        (Actor|DestroyActor _magnetstooltipactivator)))))

(event EventBeginPlay
  ;[1 1 1] Begin Play
  (|EnableCameraRotationforHMD)
  (|DetachCameraFromCapsule)
  (|DetachInstructionTextFromCapsule)
  (|DetachScoreTextFromCapsule)
  (|ActivateTooltips)
  (Utilities|SetWorldLocationandRotationAlongCurrentSpline))

(event EventTick
  (params (DeltaSeconds :type Float%20%28single-precision%29))
  ;[1 1 1] Per Frame Operations
  (|SetCameratoCurrentHeightofCapsule)
  (|RotateCameratoPointatPlayer)
  (|RotateandLocateInstructionTexttoPointatCamera
    (:Next
      (|RotateandLocateScoreTexttoPointatCamera)
      (|UpdateScore)
      (Utilities|SetWorldLocationandRotationAlongCurrentSpline))))

(event Input|ActionEvents|InputActionJump
  (params (Key :type Key%20Structure :default "AnyKey"))
  ;[1 1 1] Movement Related
  (:Pressed
    (Character|Jump)
    (CallFunction|DetachfromSpline)))

(event Input|ActionEvents|InputActionDuck
  (params (Key :type Key%20Structure :default "AnyKey"))
  ;[1 1 1] Movement Related
  (:Pressed
    (Character|Crouch))
  (:Released
    (Character|UnCrouch)))

(event Input|ActionEvents|InputActionResetVR
  (params (Key :type Key%20Structure :default "AnyKey"))
  ;[1 1 1] Movement Related
  (:Pressed
    (Class|HeadMountedDisplayFunctionLibrary|ResetOrientationandPosition 0.0 "OrientationAndPosition")))

(event Input|ActionEvents|InputActionDebugToggleFly
  (params (Key :type Key%20Structure :default "AnyKey"))
  (bind _charactermovement (Variables|Character|GetCharacterMovement))
  ;[1 1 1] Mouse input: Debug
  (:Pressed
    (switch Utilities|FlowControl|Switch|SwitchonEMovementMode (Variables|/Script/Engine.CharacterMovementComponent|GetMovementMode (Variables|Character|GetCharacterMovement))
      (:MOVE_Walking
        (Pawn|Components|CharacterMovement|SetMovementMode _charactermovement "MOVE_Flying" 0))
      (:MOVE_Flying
        (Pawn|Components|CharacterMovement|SetMovementMode _charactermovement "MOVE_Walking" 0)))))

(event Input|ActionEvents|InputActionDebugToggleMouse
  (params (Key :type Key%20Structure :default "AnyKey"))
  (bind _camera (Variables|Default|GetCamera))
  ;[1 1 1] Mouse input: Debug
  (:Pressed
    (Variables|/Script/Engine.CameraComponent|SetbUsePawnControlRotation _camera (not (Variables|/Script/Engine.CameraComponent|GetbUsePawnControlRotation _camera)))))

(event Input|AxisEvents|InputAxisMoveLeft
  (params (AxisValue :type Float%20%28single-precision%29))
  ;[1 1 1] Movement Related
  (Utilities|IsThereACurrentSplinetoFollow
    (:Yes
      (|AlterInterpolatedSplineValue AxisValue))
    (:No
      _))
  (|ExecuteLeftRightRun AxisValue))

(event Input|AxisEvents|InputAxisLookUp
  (params (AxisValue :type Float%20%28single-precision%29))
  ;[1 1 1] Mouse input: Debug
  (Pawn|Input|AddControllerPitchInput AxisValue))

(event Input|AxisEvents|InputAxisTurn
  (params (AxisValue :type Float%20%28single-precision%29))
  ;[1 1 1] Mouse input: Debug
  (Pawn|Input|AddControllerYawInput AxisValue))

(event Input|AxisEvents|InputAxisFlyUp_Test
  (params (AxisValue :type Float%20%28single-precision%29))
  ;[1 1 1] Mouse input: Debug
  (Pawn|Input|AddMovementInput "0, 0,20.000000" AxisValue false))

(event Input|AxisEvents|InputAxisMoveForward
  (params (AxisValue :type Float%20%28single-precision%29))
  ;[1 1 1] Movement Related
  (Utilities|IsThereACurrentSplinetoFollow
    (:Yes
      _)
    (:No
      _))
  (|ExecuteForwardBackwardsRun AxisValue))

(event Input|KeyboardEvents|1
  (params (Key :type Key%20Structure :default "AnyKey"))
  ;[1 1 1] Debug: Spawning Powerup
  (:Pressed
    (Development|PrintString "Magnet")
    (Game|SpawnActorfromClass "/Game/Blueprints/Environment/Pickup/BP_Magnet.BP_Magnet_C" (Transformation|GetActorTransform) "Undefined" 0 0)))

(fn ConstructionScript)

(fn OutputDistanceAlongSpline
  (params (Spline :type BP%20Spline%20Single%20Mesh%20Platform%20Object%20Reference) (Number_Of_Samples :type Float%20%28single-precision%29))
  (LocalVariables|SetSuppliedSpline (Variables|/Game/Blueprints/Environment/Spline/BP_Spline_Single_Mesh_Platform.BP_Spline_Single_Mesh_Platform_C|GetSpline Spline))
  (LocalVariables|SetNumberOfSamples Number_Of_Samples)
  (LocalVariables|SetLocationAlongSpline (|CalculateClosestDistanceonSplinetoCurrentLocation))
  (while (< (LocalVariables|GetRecordedDistanceAlongSpline) (Spline|GetSplineLength (LocalVariables|GetSuppliedSpline)))
    (if (< (Math|Float|Sqrt (Math|Float|Square (Math|Vector|DotProduct (- (Spline|GetLocationatDistanceAlongSpline (LocalVariables|GetSuppliedSpline) (LocalVariables|GetRecordedDistanceAlongSpline) "World") (LocalVariables|GetLocationAlongSpline)) (- (Spline|GetLocationatDistanceAlongSpline (LocalVariables|GetSuppliedSpline) (LocalVariables|GetRecordedDistanceAlongSpline) "World") (LocalVariables|GetLocationAlongSpline))))) (LocalVariables|GetLowestDisplacementThusFar))
      (LocalVariables|SetLowestDisplacementThusFar (Math|Float|Sqrt (Math|Float|Square (Math|Vector|DotProduct (- (Spline|GetLocationatDistanceAlongSpline (LocalVariables|GetSuppliedSpline) (LocalVariables|GetRecordedDistanceAlongSpline) "World") (LocalVariables|GetLocationAlongSpline)) (- (Spline|GetLocationatDistanceAlongSpline (LocalVariables|GetSuppliedSpline) (LocalVariables|GetRecordedDistanceAlongSpline) "World") (LocalVariables|GetLocationAlongSpline))))))
      (LocalVariables|SetDistanceWhichHasLowestDisplacementThusFar (LocalVariables|GetRecordedDistanceAlongSpline)))
    (|IncrementRecordedDistanceAlongSpline))
  (return (LocalVariables|GetDistanceWhichHasLowestDisplacementThusFar) (Spline|GetLocationatDistanceAlongSpline (LocalVariables|GetSuppliedSpline) (LocalVariables|GetDistanceWhichHasLowestDisplacementThusFar) "World")))

(fn AddScore
  (params (ScoreToAdd :type Float%20%28single-precision%29))
  ;[1 1 1] Validates input. Do nothing if score to add is negative
  (if (> ScoreToAdd 0.0)
    ;[1 1 1] Increases score
    (bind _output_get (Variables|Default|SetScore (+ ScoreToAdd (Variables|Default|GetScore))))
    ;[1 1 1] Triggers display update
    (Rendering|Components|TextRender|SetText (Variables|Default|GetScoreText) (Utilities|Text|ToText(Float) _output_get "HalfToEven" true 1 324 0 0))
    ;[1 1 1] Instruction becomes hidden once score reaches 200
    (CallFunction|InstructionVisibility)))

(fn InstructionVisibility
  (if (not (< (Variables|Default|GetScore) 2e+02))
    (Rendering|SetVisibility (Variables|Default|GetInstructionText) false false)))