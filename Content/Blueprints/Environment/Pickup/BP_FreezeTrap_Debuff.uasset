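; Debuff actor for the freeze trap pickup that holds its attached pawn frozen in place for a set duration.
; On BeginPlay it saves the pawn's velocity and gravity scale, zeroes both and deactivates its CharacterMovement.
; After the delay it restores those values, reactivates movement, spawns an ice-break particle effect at its own location and destroys itself.
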(event `self.ReceiveBeginPlay`
  (bind _charactermovement (`Character.CharacterMovement` (`self.AttachedPawn`)))
  (bind _charactermovement_2 (`Character.CharacterMovement` (`self.AttachedPawn`)))
  (bind _charactermovement_3 (`Character.CharacterMovement` (`self.AttachedPawn`)))
  (`|ExecutionSequence`
    (:`then_0`
      ;[1 1 1] Save Pawn Initial Velocity and Gravity
      (set `self.PawnInitialVelocity` (`MovementComponent.Velocity` _charactermovement_2))
      (set `self.PawnInitialGravity` (`CharacterMovementComponent.GravityScale` _charactermovement_2)))
    (:`then_1`
      ;[1 1 1] Freeze
      (set `CharacterMovementComponent.GravityScale` 0.0 _charactermovement)
      (set `MovementComponent.Velocity` (0.0 0.0 0.0) _charactermovement)
      (`ActorComponent.Deactivate` _charactermovement))
    (:`then_2`
      ;[1 1 1] Unfreeze
      (`KismetSystemLibrary.Delay` (`self.Duration`))
      (set `CharacterMovementComponent.GravityScale` (`self.PawnInitialGravity`) _charactermovement_3)
      (set `MovementComponent.Velocity` (`self.PawnInitialVelocity`) _charactermovement_3)
      (`ActorComponent.Activate` _charactermovement_3 false)
      ;[1 1 1] Destroy Debuff
      (`GameplayStatics.SpawnEmitterAtLocation` "/Game/Assets/InfinityBladeEffects/Effects/FX_Mobile/ICE/combat/P_IceTrap_Break.P_IceTrap_Break" (`self.K2_GetActorLocation`))
      (`self.K2_DestroyActor`))))

(fn `UserConstructionScript`)