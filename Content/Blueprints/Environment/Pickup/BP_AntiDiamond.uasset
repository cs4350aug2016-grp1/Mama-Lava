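; BP_AntiDiamond is a pickup that adds its ScoreGain to the activating pawn's score.
; Its DoAction event also plays a quiet, low-pitched score sound and spawns a spark particle effect at the pickup's location.
; The construction script only calls the parent's, leaving disconnected nodes that would tint a dynamic diamond material black.
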(event `self.DoAction`
  (bind _returnvalue (`self.K2_GetActorLocation`))
  ;[1 1 1] When pawn activates this coin
  (`/Game/Blueprints/Character/BP_MamaLava_Player.AddScore` (`self.Pawn`) (`self.ScoreGain`))
  (`GameplayStatics.PlaySoundAtLocation` "/Game/Assets/StarterContent/Audio/SFX_Score_01.SFX_Score_01" _returnvalue (struct) 0.2 0.2)
  (`GameplayStatics.SpawnEmitterAtLocation` "/Game/Assets/InfinityBladeEffects/Effects/FX_Monsters/FX_Monster_Ausar/P_AU_Taunt_sparks.P_AU_Taunt_sparks" _returnvalue))

(fn `UserConstructionScript`
  (`parent.UserConstructionScript`))