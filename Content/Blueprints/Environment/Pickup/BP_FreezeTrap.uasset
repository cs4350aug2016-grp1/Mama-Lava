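; BP_FreezeTrap is a pickup whose action applies a freeze debuff to a pawn.
; DoAction spawns a BP_FreezeTrap_Debuff at the pawn's ChestPoint, passing the freeze duration and the pawn.
; The debuff's root uses absolute rotation and scale, then attaches to the pawn so it follows position only.
; The construction script only calls the parent implementation.
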(event `self.DoAction`
  ;[1 1 1] Create and attach a FreezeTrap debuff
  (bind _returnvalue (`|SpawnActorFromClass` "/Game/Blueprints/Environment/Pickup/BP_FreezeTrap_Debuff.BP_FreezeTrap_Debuff_C" (`SceneComponent.K2_GetComponentToWorld` (`/Game/Blueprints/Character/BP_MamaLava_Player.ChestPoint` (`self.Pawn`))) "Undefined" "OverrideRootScale" null (`self.FreezeDuration`) (`self.Pawn`)))
  (`SceneComponent.SetAbsolute` (`/Game/Blueprints/Environment/Pickup/BP_FreezeTrap_Debuff.DefaultSceneRoot` _returnvalue) false true true)
  (`self.K2_AttachToActor` _returnvalue (`self.Pawn`) "None" "KeepWorld" "KeepWorld" "KeepWorld" false))

(fn `UserConstructionScript`
  (`parent.UserConstructionScript`))