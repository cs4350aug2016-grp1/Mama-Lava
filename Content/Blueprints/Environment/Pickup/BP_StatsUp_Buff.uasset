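; Stat-up buff actor that expires after a set duration and restores its attached pawn's movement stats.
; BeginPlay starts a one-shot timer that fires two seconds short of Duration, clamped at zero.
; A timeline macro then shrinks the root to zero scale before jump velocity and max walk speed return to base values.
; A fire-off particle effect plays at its location as the actor destroys itself.
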(event `self.ReceiveBeginPlay`
  (`self.SetLifeSpanTimer`))

(event `SetLifeSpanTimer`
  (`KismetSystemLibrary.K2_SetTimerDelegate` (delegate `BeginDestroy`) (`KismetMathLibrary.FMax` (- (`self.Duration`) 2.0))))

(event `BeginDestroy`
  (bind _attachedpawn (`self.AttachedPawn`))
  (bind _attachedpawn_2 (`self.AttachedPawn`))
  (bind (_direction _value) (`Timeline|ScaleValue` :!via `PlayFromStart`)
    (:`Update`
      (`SceneComponent.SetWorldScale3D` (`self.DefaultSceneRoot`) (`KismetMathLibrary.VLerp` (`SceneComponent.K2_GetComponentScale` (`self.DefaultSceneRoot`)) (0.0 0.0 0.0) _value)))
    (:`Finished`
      (set `CharacterMovementComponent.JumpZVelocity` (`/Game/Blueprints/Character/BP_MamaLava_Player.BaseJumpingZVelocity` _attachedpawn) (`Character.CharacterMovement` _attachedpawn))
      (set `CharacterMovementComponent.MaxWalkSpeed` (`/Game/Blueprints/Character/BP_MamaLava_Player.BaseMaxWalkSpeed` _attachedpawn_2) (`Character.CharacterMovement` _attachedpawn_2))
      (`GameplayStatics.SpawnEmitterAtLocation` "/Game/Assets/InfinityBladeEffects/Effects/FX_Mobile/Fire/combat/P_Trap_Fire_Grate_Off.P_Trap_Fire_Grate_Off" (`self.K2_GetActorLocation` self))
      (`self.K2_DestroyActor`))))

(fn `UserConstructionScript`)