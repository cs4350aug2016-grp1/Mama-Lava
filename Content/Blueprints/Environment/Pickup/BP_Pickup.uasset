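; Base pickup actor for MamaLava that triggers an action when the player overlaps it, then destroys itself.
; Sphere overlap accepts only the game mode's default pawn class, runs the empty DoAction hook, then tells the player to disable the tooltip for its activator class.
; ShowTooltip reveals the text and selection indicator once, detaching the text and yawing it toward the world's vertical axis at the origin.
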(event `Show Tooltip`
  (params (Tooltip :type Text))
  (bind _returnvalue (+ (`self.K2_GetActorLocation`) (`SceneComponent.K2_GetComponentLocation` (`self.TooltipText`))))
  ;[1 1 1] Set tool tip
  (`/Engine/EditorBlueprintResources/StandardMacros.DoOnce` false
    (:`Completed`
      (`|ExecutionSequence`
        (:`then_0`
          (`SceneComponent.SetVisibility` (`self.TooltipText`) true false)
          (`TextRenderComponent.K2_SetText` (`self.TooltipText`) Tooltip)
          (`SceneComponent.K2_DetachFromComponent` (`self.TooltipText`) "KeepRelative" "KeepRelative" "KeepRelative" true)
          (`SceneComponent.K2_SetWorldLocationAndRotation` (`self.TooltipText`) _returnvalue (`KismetMathLibrary.FindLookAtRotation` _returnvalue (`KismetMathLibrary.MakeVector` 0.0 0.0 (.z _returnvalue))) false false))
        (:`then_1`
          (`SceneComponent.SetVisibility` (`self.TooltipSelectionIndicator`) true false))))))

(event `self.SphereCollision.OnComponentBeginOverlap`
  (params (OverlappedComponent :type "PrimitiveComponent Object Reference") (OtherActor :type "Actor Object Reference") (OtherComp :type "PrimitiveComponent Object Reference") (OtherBodyIndex :type Integer) (bFromSweep :type Boolean) (SweepResult :type "HitResult Structure (by ref)"))
  (bind _istrue (`self.IsDefaultPawnClass` OtherActor))
  (if _istrue
    (set `self.Pawn` (cast `/Game/Blueprints/Character/BP_MamaLava_Player` OtherActor :!pure true))
    (`self.DoAction`)
    (`self.DisableTooltip`)
    (`self.K2_DestroyActor`)))

(event `DoAction`)

(event `DisableTooltip`
  (`/Engine/EditorBlueprintResources/StandardMacros.DoOnce` false
    (:`Completed`
      (`/Game/Blueprints/Character/BP_MamaLava_Player.DisableTooltip` (`self.Pawn`) (`self.TooltipActivatorClass`)))))

(fn `GetMainGameMode`
  (returns (MainGameMode :type "/Game/GameHandlers/BP_MamaLava_GameMode Object Reference"))
  (return (cast `/Game/GameHandlers/BP_MamaLava_GameMode` (`GameplayStatics.GetGameMode`) :!pure true)))

(fn `IsDefaultPawnClass`
  (params (ActorToCheck :type "Actor Object Reference"))
  (returns (IsTrue :type Boolean))
  (bind _maingamemode (`self.GetMainGameMode`))
  (return (== (`GameMode.DefaultPawnClass` _maingamemode) (`GameplayStatics.GetObjectClass` ActorToCheck))))

(fn `UserConstructionScript`
  (`parent.UserConstructionScript`))