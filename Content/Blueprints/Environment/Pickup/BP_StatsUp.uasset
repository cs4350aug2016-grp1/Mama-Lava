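; BP_StatsUp is a pickup that temporarily boosts the pawn's jump velocity and max walk speed by a buff factor.
; On activation it plays an effect and searches the pawn's attached actors for a BP_StatsUp_Buff.
; An existing buff gets its lifespan timer refreshed; otherwise it scales base stats and attaches a new buff.
; A buff pending destruction is told not to reset stats, then replaced.
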(event `self.DoAction`
  (set `self.CharacterMovement` (`Character.CharacterMovement` (`self.Pawn`)))
  (`GameplayStatics.SpawnEmitterAtLocation` "/Game/Assets/Pickups/ParticleSystems/P_StatsUpPickupEffect.P_StatsUpPickupEffect" (`self.K2_GetActorLocation`))
  (bind (_doesexist _buff) (`self.CheckExistingBuff`))
  (if _doesexist
    ;[1 1 1] Refresh duration current Buff if it is not pending kill. Otherwise just do not reset stats and create a new Buff
    (`/Engine/EditorBlueprintResources/StandardMacros.IsValid` _buff
      (:`Is Valid`
        (if (`/Game/Blueprints/Environment/Pickup/BP_StatsUp_Buff.IsPendingDestroy` _buff)
          (`/Engine/EditorBlueprintResources/StandardMacros.IsValid` _buff
            (:`Is Valid`
              (set `/Game/Blueprints/Environment/Pickup/BP_StatsUp_Buff.ShouldResetStats` false _buff)
              (`self.CreateNewBuff`)))
          (else
            (`/Game/Blueprints/Environment/Pickup/BP_StatsUp_Buff.SetLifeSpanTimer` _buff)))))
    (else
      ;[1 1 1] Otherwise just create a new Buff
      (`self.CreateNewBuff`))))

(event `CreateNewBuff`
  ;[1 1 1] Create a new Buff
  (`|ExecutionSequence`
    (:`then_0`
      ;;[1 1 1] Buff Jump Z Velocity
      (set `CharacterMovementComponent.JumpZVelocity` (* (`/Game/Blueprints/Character/BP_MamaLava_Player.BaseJumpingZVelocity` (`self.Pawn`)) (`self.BuffFactor`)) (`self.CharacterMovement`)))
    (:`then_1`
      ;;[1 1 1] Buff Max Walk Speed
      (set `CharacterMovementComponent.MaxWalkSpeed` (* (`/Game/Blueprints/Character/BP_MamaLava_Player.BaseMaxWalkSpeed` (`self.Pawn`)) (`self.BuffFactor`)) (`self.CharacterMovement`)))
    (:`then_2`
      (bind _returnvalue (`|SpawnActorFromClass` "/Game/Blueprints/Environment/Pickup/BP_StatsUp_Buff.BP_StatsUp_Buff_C" (`SceneComponent.K2_GetComponentToWorld` (`/Game/Blueprints/Character/BP_MamaLava_Player.ChestPoint` (`self.Pawn`))) "Undefined" "OverrideRootScale" null (`self.BuffDuration`) (`self.Pawn`)))
      (`SceneComponent.SetAbsolute` (`/Game/Blueprints/Environment/Pickup/BP_StatsUp_Buff.DefaultSceneRoot` _returnvalue) false true true)
      (`self.K2_AttachToActor` _returnvalue (`self.Pawn`) "None" "KeepWorld" "KeepWorld" "KeepWorld" true))))

(fn `CheckExistingBuff`
  (returns (DoesExist :type Boolean) (Buff :type "/Game/Blueprints/Environment/Pickup/BP_StatsUp_Buff Object Reference"))
  (for _array_element (`self.GetAttachedActors` (`self.Pawn`))
    (bind _asbp_stats_up_buff (cast `/Game/Blueprints/Environment/Pickup/BP_StatsUp_Buff` _array_element))
    (return true _asbp_stats_up_buff))
  (return false null))

(fn `UserConstructionScript`
  (`parent.UserConstructionScript`))