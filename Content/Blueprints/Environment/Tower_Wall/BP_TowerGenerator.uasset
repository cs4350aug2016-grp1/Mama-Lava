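; Builds a tower at construction time by chaining four BP_Tower_Segment child actors, each placed at the previous segment's attach transform.
; Segment constants define a ring spline of equal unit-length steps inside the wall.
; A fixed stretch of that spline is sampled in world space for each segment.
; Wooden platform child actors are added to the segment, their spline meshes bent between consecutive samples.
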(event EventBeginPlay)

(fn ConstructionScript
  (CallFunction|InitializePlatformGenerator)
  (for _index (range 0 3)
    (bind _returnvalue (AddComponent|AddChildActorComponent false (Variables|Default|GetNextSpawnPoint)))
    (bind _asbp_tower_segment (Utilities|Casting|CastToBP_Tower_Segment (Variables|/Script/Engine.ChildActorComponent|GetChildActor _returnvalue)))
    (bind _output_get (LocalVariables|SetCurrentSegment _asbp_tower_segment))
    (bind _ref (Default|InitializeProperties _output_get (Variables|TowerSegment|GetSegmentConstantData) false 1))
    (bind _attachtransform (Default|GetAttachTransform _ref))
    (Variables|Default|SetNextSpawnPoint _attachtransform)
    (bind _splinepointsdata (CallFunction|GenerateSplinePointsData 0.0 3e+02))
    (CallFunction|AddPlatforms (LocalVariables|GetCurrentSegment) _splinepointsdata "/Game/Blueprints/Environment/Spline/BP_Wooden_Platform_Segment.BP_Wooden_Platform_Segment_C")))

(fn AddPlatforms
  (params (OwningSegment :type BP%20Tower%20Segment%20Object%20Reference) (SplineData :type Array%20of%20S%20Spline%20Data%20Structures) (PlatformType :type BP%20Platform%20Segment%20Base%20Class%20Reference))
  (LocalVariables|SetSegment OwningSegment)
  (LocalVariables|SetSplinePts SplineData)
  (LocalVariables|SetPlatType PlatformType)
  ;[1 1 1] Create the number of spline actors and set spline data based on the main Spline component
  (for _index (range 0 (- (Utilities|Array|LastIndex (LocalVariables|GetSplinePts)) 1))
    (Utilities|FlowControl|Sequence
      (:then_0
        (bind _returnvalue (AddComponent|AddChildActorComponent (LocalVariables|GetSegment) false))
        (ChildActorComponent|SetChildActorClass _returnvalue (LocalVariables|GetPlatType))
        (bind _asbp_platform_segment_base (Utilities|Casting|CastToBP_Platform_Segment_Base (Variables|/Script/Engine.ChildActorComponent|GetChildActor _returnvalue)))
        (bind _output_get (LocalVariables|SetPlat _asbp_platform_segment_base))
        (Development|PrintString (Utilities|GetDisplayName _output_get))
        (Development|PrintString (Utilities|String|ToString(Vector) (Transformation|GetWorldLocation (Variables|/Script/Engine.SplineMeshActor|GetSplineMeshComponent _output_get)))))
      (:then_1
        ;;[1 1 1] Set current and next index
        (bind _output_get_2 (LocalVariables|SetCurPointIndex _index))
        (LocalVariables|SetNextPointIndex (+ _output_get_2 1)))
      (:then_2
        (|SetStartandEndForSplineActor))))
  (return))

(fn InitializePlatformGenerator
  (bind _unitlength (Variables|Platform|GetUnitLength))
  (bind _segmentconstantdata (Variables|TowerSegment|GetSegmentConstantData))
  (LocalVariables|SetHeight (.height _segmentconstantdata))
  (bind _output_get (Variables|Platform|SetPlatformRadius (- (.innerradius _segmentconstantdata) (/ (.platformgap _segmentconstantdata) 2.0))))
  (Variables|Platform|SetUnitAngle (/ (* (Class|KismetMathLibrary|Asin (/ _unitlength (* _output_get 2.0))) 2.0 1.8e+02) (Math|Trig|GetPI)))
  (bind _output_get_2 (Variables|Platform|SetNbSides (Math|Float|Ceil (/ (Math|Trig|GetPI) (Class|KismetMathLibrary|Asin (/ _unitlength (* _output_get 2.0)))))))
  (Variables|Platform|SetSplineLength (* _output_get_2 _unitlength))
  ;[1 1 1] Int has 32 bits, bits length = num of ints needed to encode unit side
  (Variables|Platform|SetEncodedBitsLength (Math|Float|Ceil (/ (Math|Conversions|ToFloat(Integer) (Variables|Platform|GetNbSides)) 32.0)))
  (LocalVariables|SetVect (Math|Vector|MakeVector 0.0 (Variables|Platform|GetPlatformRadius) (LocalVariables|GetHeight)))
  (Spline|ClearSplinePoints (Variables|Default|GetSpline))
  (for _index (range 1 (Variables|Platform|GetNbSides))
    (Spline|AddSplinePoint (Variables|Default|GetSpline) (LocalVariables|GetVect) "Local")
    (LocalVariables|SetVect (Math|Vector|RotateVectorAroundAxis (LocalVariables|GetVect) (Variables|Platform|GetUnitAngle) "0, 0,1.000000"))))

(fn GenerateSplinePointsData
  (params (StartDistance :type Float%20%28single-precision%29) (EndDistance :type Float%20%28single-precision%29))
  (LocalVariables|SetStart StartDistance)
  (LocalVariables|SetEnd EndDistance)
  (Utilities|Array|SetArrayElem (LocalVariables|GetSplineData) 0 (Utilities|Struct|MakeS_Spline_Data (Spline|GetLocationatDistanceAlongSpline (Variables|Default|GetSpline) (Math|Float|%(Float) (LocalVariables|GetStart) (Variables|Platform|GetSplineLength)) "World") (Spline|GetTangentatDistanceAlongSpline (Variables|Default|GetSpline) (Math|Float|%(Float) (LocalVariables|GetStart) (Variables|Platform|GetSplineLength)) "World")))
  (while (<= (+ (LocalVariables|GetCurrent) (Variables|Platform|GetUnitLength)) (LocalVariables|GetEnd))
    (bind _output_get (LocalVariables|SetCurrent (+ (LocalVariables|GetCurrent) (Variables|Platform|GetUnitLength))))
    (Utilities|Array|Add (LocalVariables|GetSplineData) (Utilities|Struct|MakeS_Spline_Data (Spline|GetLocationatDistanceAlongSpline (Variables|Default|GetSpline) (Math|Float|%(Float) _output_get (Variables|Platform|GetSplineLength)) "World") (Spline|GetTangentatDistanceAlongSpline (Variables|Default|GetSpline) (Math|Float|%(Float) _output_get (Variables|Platform|GetSplineLength)) "World"))))
  (return (LocalVariables|GetSplineData)))