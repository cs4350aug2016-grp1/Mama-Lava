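; BP_SmokeRoof is a tower roof smoke effect that follows the Mama Lava game mode's NextSpawnPoint.
; The construction script caches the game mode, and BeginPlay turns on shadow casting for the particle system.
; Each Tick lerps from NextSpawnPoint toward the root's current transform at a low fixed alpha, so the root closes most of the gap every frame, independent of delta time.
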(event `self.ReceiveBeginPlay`
  (`PrimitiveComponent.SetCastShadow` (`self.ParticleSystem`) true))

(event `self.ReceiveTick`
  (params (DeltaSeconds :type "Float (single-precision)"))
  (`SceneComponent.K2_SetWorldTransform` (`self.DefaultSceneRoot`) (`KismetMathLibrary.TLerp` (`/Game/GameHandlers/BP_MamaLava_GameMode.NextSpawnPoint` (`self.MamaLavaGameMode`)) (`SceneComponent.K2_GetComponentToWorld` (`self.DefaultSceneRoot`)) 0.15) false false))

(fn `UserConstructionScript`
  (set `self.MamaLavaGameMode` (cast `/Game/GameHandlers/BP_MamaLava_GameMode` (`GameplayStatics.GetGameMode`) :!pure true)))