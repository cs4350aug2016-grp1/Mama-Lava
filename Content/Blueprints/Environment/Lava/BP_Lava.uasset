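; BP_Lava is an environmental lava surface that triggers delayed destruction of BP_Lava_Destructible actors overlapping its trigger box.
; The construction script builds the surface from a dynamic instance of an ocean material, setting wave, displacement and tessellation parameters, then scales the actor by Radius.
; SpawnFireEffect spawns BP_Fire_Effect at a random point from the particle area, but its looping timer is disconnected and never runs.
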(event `self.ReceiveBeginPlay`)

(event `self.DestroyTriggerBox.OnComponentBeginOverlap`
  (params (OverlappedComponent :type "PrimitiveComponent Object Reference") (OtherActor :type "Actor Object Reference") (OtherComp :type "PrimitiveComponent Object Reference") (OtherBodyIndex :type Integer) (bFromSweep :type Boolean) (SweepResult :type "HitResult Structure (by ref)"))
  (bind _asbp_lava_destructible (cast `/Game/Blueprints/Environment/BP_Lava_Destructible` OtherActor))
  (`/Game/Blueprints/Environment/BP_Lava_Destructible.DestroyAfterDelay` _asbp_lava_destructible))

(fn `SpawnFireEffect`
  (bind _particlespawnarea (`self.ParticleSpawnArea`))
  ;[1 1 1] Actor has initial life span so no need to destroy
  (`|SpawnActorFromClass` "/Game/Blueprints/Environment/Lava/BP_Fire_Effect.BP_Fire_Effect_C" (`KismetMathLibrary.Conv_VectorToTransform` (+ (`KismetMathLibrary.RandomPointInBoundingBox` (`SceneComponent.RelativeLocation` _particlespawnarea) (`BoxComponent.BoxExtent` _particlespawnarea)) (`SceneComponent.K2_GetComponentLocation` _particlespawnarea))) "Undefined" "OverrideRootScale"))

(fn `UserConstructionScript`
  (bind _watersurface (`self.WaterSurface`))
  (bind _water_material (`self.Water Material`))
  (bind _returnvalue (/ (`self.Radius`) 500.0))
  (bind _returnvalue_2 (`PrimitiveComponent.CreateDynamicMaterialInstance` _watersurface 0 (`self.Ocean Material`)))
  (set `self.Water Material` _returnvalue_2)
  (`SceneComponent.SetRelativeScale3D` _watersurface (`KismetMathLibrary.MakeVector` (`self.Water Scale X`) (`self.Water Scale Y`) 1.0))
  (`MaterialInstanceDynamic.SetScalarParameterValue` _water_material "WaterSpeed" (`self.Overall Water Speed`))
  (`MaterialInstanceDynamic.SetScalarParameterValue` _water_material "WaterScale" (`self.Overall Water Scale`))
  (`MaterialInstanceDynamic.SetScalarParameterValue` _water_material "Displacement" (`self.Displacement`))
  (`MaterialInstanceDynamic.SetScalarParameterValue` _water_material "Tesselation" (`self.Tesselation Factor`))
  (`MaterialInstanceDynamic.SetScalarParameterValue` _water_material "Large Wave Amplify" (`self.Amplify Large Normals`))
  (`MaterialInstanceDynamic.SetScalarParameterValue` _water_material "Small Wave Amplify" (`self.Amplify Small Normals`))
  (`self.SetActorRelativeScale3D` (`KismetMathLibrary.MakeVector` _returnvalue _returnvalue 1.0)))