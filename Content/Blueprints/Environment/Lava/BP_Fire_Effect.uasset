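; BP_Fire_Effect is an environment actor in the lava set that places a ring of particle effects at a configurable platform radius.
; Its construction script rebuilds a circular spline by rotating an offset vector around the Z axis in 52 equal steps.
; Each step also adds a particle system component at the rotated position, using the ChildEffect template.
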(fn `UserConstructionScript`
  ;[1 1 1] Create spline points
  (set `self.Vect` (`KismetMathLibrary.MakeVector` 0.0 (`self.PlatformRadius`)))
  (`SplineComponent.ClearSplinePoints` (`self.Spline`))
  (for _ (range 1 53)
    (`SplineComponent.AddSplinePoint` (`self.Spline`) (`self.Vect`) "Local")
    (bind _output_get (set `self.Vect` (`KismetMathLibrary.RotateAngleAxis` (`self.Vect`) (/ 360.0 52.0) (0.0 0.0 1.0))))
    (bind _returnvalue (`AddComponent|Particle System Component_0` :`RelativeTransform` (`KismetMathLibrary.Conv_VectorToTransform` _output_get)))
    (`ParticleSystemComponent.SetTemplate` _returnvalue (`self.ChildEffect`))))