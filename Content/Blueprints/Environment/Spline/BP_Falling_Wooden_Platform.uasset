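; Spline-mesh wooden platform on a tower segment that falls under physics and can be reset.
; Action saves the mesh's offset from its TowerSegment, enables physics, darkens the dynamic material and calls EventRevertAction.
; InverseAction stops physics and collision and rebuilds the transform from that offset, then LavaDestructionAfterDelay restores opacity, color and collision.
; ExecutePlayerMiniJump gives a grounded player a reduced-velocity hop.
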(event EventAction
  (Variables|Default|SetActionDone false)
  (CallFunction|UpdateRelativeOffsetfromTowerSegment)
  (Utilities|CheckSelfValidity
    (:True
      (Physics|SetSimulatePhysics (Variables|Default|GetSplineMeshComponent) true)
      (Rendering|Material|SetVectorParameterValue (Variables|Default|GetDMI) "Color" (* (Variables|Default|GetColor) 0.2) :!class /Script/Engine.MaterialInstanceDynamic)
      (CallFunction|EventRevertAction))))

(event EventInverseAction
  (Utilities|CheckSelfValidity
    (:True
      (Physics|SetSimulatePhysics (Variables|Default|GetSplineMeshComponent) false)
      (Utilities|CheckSelfValidity
        (:True
          (Collision|SetCollisionEnabled (Variables|Default|GetSplineMeshComponent) "NoCollision")
          (bind _returnvalue (CallFunction|ObtainResetTransform))
          (Utilities|CheckSelfValidity
            (:True
              (Transformation|SetWorldTransform (Variables|Default|GetSplineMeshComponent) _returnvalue false false)
              (Variables|Default|SetActionDone true))))))))

(event EventLavaDestructionAfterDelay
  (if (Variables|Default|GetActionDone)
    _
    (else
      (Utilities|FlowControl|Delay 0.1)))
  (Rendering|Material|SetScalarParameterValue (Variables|Default|GetDMI) "Opacity" 1.0 :!class /Script/Engine.MaterialInstanceDynamic)
  (Utilities|CheckSelfValidity
    (:True
      (Rendering|Material|SetVectorParameterValue (Variables|Default|GetDMI) "Color" (Variables|Default|GetColor) :!class /Script/Engine.MaterialInstanceDynamic)
      (Utilities|CheckSelfValidity
        (:True
          (Collision|SetCollisionEnabled (Variables|Default|GetSplineMeshComponent) "QueryAndPhysics"))))))

(fn ConstructionScript
  (|CallParentFunction)
  (|CreateDMI)
  (|SaveColorofPlatform))

(fn ExecutePlayerMiniJump
  (params (Object :type Object%20Object%20Reference))
  (bind _asbp_mama_lava_player (Utilities|Casting|CastToBP_MamaLava_Player Object)
    (:then
      (bind _output_get (LocalVariables|SetCurrPlayer _asbp_mama_lava_player))
      (|isOnGround _output_get
        (:True
          (Utilities|FlowControl|Sequence
            (:then_0
              (LocalVariables|SetPlayerBaseJump (Variables|/Game/Blueprints/Character/BP_MamaLava_Player.BP_MamaLava_Player_C|GetBaseJumpingZVelocity (LocalVariables|GetCurrPlayer))))
            (:then_1
              (Variables|/Game/Blueprints/Character/BP_MamaLava_Player.BP_MamaLava_Player_C|SetBaseJumpingZVelocity (LocalVariables|GetCurrPlayer) (* (LocalVariables|GetPlayerBaseJump) 0.4)))
            (:then_2
              (Character|Jump (LocalVariables|GetCurrPlayer)))
            (:then_3
              (Variables|/Game/Blueprints/Character/BP_MamaLava_Player.BP_MamaLava_Player_C|SetBaseJumpingZVelocity (LocalVariables|GetCurrPlayer) (LocalVariables|GetPlayerBaseJump)))
            (:then_4
              (return))))
        (:false
          (return))))
    (:CastFailed
      (return))))

(fn UpdateRelativeOffsetfromTowerSegment
  (bind _splinemeshcomponent (Variables|Default|GetSplineMeshComponent))
  (bind _returnvalue (Transformation|GetWorldTransform _splinemeshcomponent))
  (bind _towersegment (Utilities|GetTowerSegment))
  (Variables|Default|SetLocationOffset (- (.location (Transformation|GetWorldTransform (VehicleSound|GetRootComponent _towersegment))) (.location _returnvalue)))
  (Variables|Default|SetRotatorOffset (Math|Rotator|Delta(Rotator) (.rotation (Transformation|GetWorldTransform (VehicleSound|GetRootComponent _towersegment))) (.rotation _returnvalue)))
  (Variables|Default|SetScaleOffset (- (.scale (Transformation|GetWorldTransform (VehicleSound|GetRootComponent _towersegment))) (.scale _returnvalue)))
  (return))

(fn ObtainResetTransform
  (bind _towersegment (Utilities|GetTowerSegment))
  (return (Math|Transform|MakeTransform (- (.location (Transformation|GetWorldTransform (VehicleSound|GetRootComponent _towersegment))) (Variables|Default|GetLocationOffset)) (Class|KismetMathLibrary|NegateRotator (Variables|Default|GetRotatorOffset)) (- (.scale (Transformation|GetWorldTransform (VehicleSound|GetRootComponent _towersegment))) (Variables|Default|GetScaleOffset)))))