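; Old spline platform generator actor: GeneratePlatforms takes a spline and segment class to build platforms from spline mesh segment actors.
; CreateActorsInReferenceArray spawns segments at its root and shapes each between consecutive spline points using local locations and tangents, wrapping at the end.
; GetNumberOfSplineMeshActorsToGenerate sets the loop bound, but its closed-loop-aware calculation is unconnected.
; Reference-array tracking and cleanup are unused; the cleanup function only clears the array.
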(event `Event Generate Platforms`
  (params (Spline_Curve :type "SplineComponent Object Reference") (Segment_Class_To_Spawn :type "Actor Class Reference") (NewParam :type Boolean))
  (set `self.SplineCurve` Spline_Curve)
  (set `self.SegmentClassToSpawn` Segment_Class_To_Spawn)
  (`self.CreateActorsInReferenceArray`))

(fn `CreateActorsInReferenceArray`
  (locals (CurrentSplineMeshActor :type "/Game/Blueprints/Environment/Spline/Old/BP_Spline_Mesh_Platform_Segment_Actor_Base Object Reference") (CurrentPointIndex :type Integer) (NextPointIndex :type Integer))
  (for _index (range (+ (`self.GetNumberOfSplineMeshActorsToGenerate`) 1))
    (`|ExecutionSequence`
      (:`then_0`
        (bind _returnvalue (`|SpawnActorFromClass` (`self.SegmentClassToSpawn`) (`SceneComponent.K2_GetComponentToWorld` (`self.DefaultSceneRoot`)) "AlwaysSpawn" "OverrideRootScale" self))
        (bind _asbp_spline_mesh_platform_segment_actor_base (cast `/Game/Blueprints/Environment/Spline/Old/BP_Spline_Mesh_Platform_Segment_Actor_Base` _returnvalue)
          (:`then`
            (set `local.CurrentSplineMeshActor` _asbp_spline_mesh_platform_segment_actor_base))
          (:`CastFailed`
            (return))))
      (:`then_1`
        (bind _output_get (set `local.CurrentPointIndex` _index))
        (set `local.NextPointIndex` (mod (+ _output_get 1) (`SplineComponent.GetNumberOfSplinePoints` (`self.SplineCurve`))))
        (`|ExecutionSequence`
          (:`then_0`
            (`SplineMeshComponent.SetStartAndEnd` (`SplineMeshActor.SplineMeshComponent` (`local.CurrentSplineMeshActor`)) (`SplineComponent.GetLocationAtSplinePoint` (`self.SplineCurve`) (`local.CurrentPointIndex`) "Local") (`SplineComponent.GetTangentAtSplinePoint` (`self.SplineCurve`) (`local.CurrentPointIndex`) "Local") (`SplineComponent.GetLocationAtSplinePoint` (`self.SplineCurve`) (`local.NextPointIndex`) "Local") (`SplineComponent.GetTangentAtSplinePoint` (`self.SplineCurve`) (`local.NextPointIndex`) "Local") true))))))
  (return))

(fn `DestroyActorsInReferenceArray`
  (for _array_element (`self.SplineMeshActorReferenceArray`)
    (cast `/Game/Blueprints/Environment/Spline/Old/BP_Spline_Mesh_Platform_Segment_Actor_Base` _array_element))
  (`KismetArrayLibrary.Array_Clear` (`self.SplineMeshActorReferenceArray`))
  (return))

(fn `UserConstructionScript`
  (`parent.UserConstructionScript`))