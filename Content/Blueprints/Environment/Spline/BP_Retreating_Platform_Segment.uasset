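; Spline-mesh platform segment for the MamaLava game mode that slides back and forth along a direction vector.
; On BeginPlay it sets an Origin from either the PlatformGenerator or a fixed point, based on spline start X, then gets Direction from GetDirectionVector.
; A looping timer runs Update instead of Tick, stepping the local offset and reversing Direction after a fixed step count.
; GetDirectionVector's graph holds only an unused origin-to-midpoint calculation.
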(event `self.ReceiveBeginPlay`
  (bind _returnvalue_x (`KismetMathLibrary.BreakVector` (`SplineMeshComponent.GetStartPosition` (`self.SplineMeshComponent`))))
  (`|ExecutionSequence`
    (:`then_0`
      (bind _asbp_mama_lava_game_mode (cast `/Game/GameHandlers/BP_MamaLava_GameMode` (`GameplayStatics.GetGameMode`))))
    (:`then_1`
      (if (> _returnvalue_x 1000.0)
        (set `self.Origin` (4500.0 0.0 0.0))
        (else
          (bind (_returnvalue_x_2 _returnvalue_y) (`KismetMathLibrary.BreakVector` (`self.K2_GetActorLocation` (`/Game/GameHandlers/BP_MamaLava_GameMode.PlatformGenerator` _asbp_mama_lava_game_mode))))
          (set `self.Origin` (`KismetMathLibrary.MakeVector` _returnvalue_x_2 _returnvalue_y)))))
    (:`then_2`
      (set `self.Direction` (`self.GetDirectionVector`)))
    (:`then_3`
      (`KismetSystemLibrary.K2_SetTimer` null "Update" 0.1 true))))

(event `self.ReceiveTick`
  (params (DeltaSeconds :type "Float (single-precision)")))

(fn `Update`
  (if (< (`self.Count`) 20)
    (`/Engine/EditorBlueprintResources/StandardMacros.IncrementInt` (`self.Count`)
      (:`  `
        _))
    (else
      (set `self.Direction` (`KismetMathLibrary.NegateVector` (`self.Direction`)))
      (set `self.Count` 1)))
  (`self.K2_AddActorLocalOffset` (* (`self.Direction`) 6))
  (return))

(fn `UserConstructionScript`
  (`parent.UserConstructionScript`))