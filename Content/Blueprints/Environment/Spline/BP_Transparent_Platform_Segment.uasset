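; Spline-mesh platform segment that fades its brick material and is passable while mostly transparent.
; The construction script runs the parent's script, then puts a dynamic transparency material instance on the spline mesh.
; From BeginPlay, the Opacity timeline drives that material's opacity parameter and switches actor collision off below a threshold and back on otherwise.
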(event `self.ReceiveBeginPlay`
  (bind (_direction _data) (`Timeline|Opacity`)
    (:`Update`
      (`MaterialInstanceDynamic.SetScalarParameterValue` (`self.Opacity_index`) "Opacity" _data)
      (if (< _data 0.3)
        (if (`self.GetActorEnableCollision`)
          (`self.SetActorEnableCollision` false))
        (elif (not (`self.GetActorEnableCollision`))
          (`self.SetActorEnableCollision` true))))))

(fn `UserConstructionScript`
  (`parent.UserConstructionScript`)
  (bind _returnvalue (`PrimitiveComponent.CreateDynamicMaterialInstance` (`self.SplineMeshComponent`) 0 "/Game/Assets/StarterContent/Materials/M_Brick_Transparency.M_Brick_Transparency"))
  (set `self.Opacity_index` _returnvalue))