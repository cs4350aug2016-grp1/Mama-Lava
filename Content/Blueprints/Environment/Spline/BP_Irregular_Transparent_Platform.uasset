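; Spline mesh platform whose opacity changes over time and which loses collision while mostly transparent.
; The construction script runs the parent's logic, then creates a dynamic instance of the purple wooden platform material on the spline mesh.
; After a random delay of up to a second at BeginPlay, a timeline drives that material's Opacity parameter.
; Actor collision switches off below an opacity threshold and back on otherwise, only when the state needs changing.
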(event `self.ReceiveBeginPlay`
  (`KismetSystemLibrary.Delay` (`KismetMathLibrary.RandomFloatInRange` 0.0 1.0))
  (bind (_direction _data) (`Timeline|Opacity` :!via `PlayFromStart`)
    (:`Update`
      (`MaterialInstanceDynamic.SetScalarParameterValue` (`self.Opacity_index`) "Opacity" _data)
      (if (< _data 0.3)
        (if (`self.GetActorEnableCollision`)
          (`self.SetActorEnableCollision` false))
        (elif (not (`self.GetActorEnableCollision`))
          (`self.SetActorEnableCollision` true))))))

(fn `UserConstructionScript`
  (`parent.UserConstructionScript`)
  (bind _returnvalue (`PrimitiveComponent.CreateDynamicMaterialInstance` (`self.SplineMeshComponent`) 0 "/Game/Assets/Environment/WoodenPlatform/Materials/MI_Wooden_Platform_Purple.MI_Wooden_Platform_Purple"))
  (set `self.Opacity_index` _returnvalue))