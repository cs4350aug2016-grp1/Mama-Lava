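; Base Blueprint for spline platform segments that trigger a one-time action.
; ExecuteAction passes through a DoOnce, waits for the supplied delay, then calls Action, which is left empty here.
; Helper functions fetch overlapping BP_MamaLava_Player actors and test whether a given object is that player class.
; Construction only runs the parent's script.
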(event `Event ExecuteAction`
  (params (Delay :type "Float (double-precision)"))
  (`/Engine/EditorBlueprintResources/StandardMacros.DoOnce` false
    (:`Completed`
      (`KismetSystemLibrary.Delay` Delay)
      (`self.Action`))))

(fn `Action`)

(fn `getAllOverlappingPlayers`
  (returns (`Overlapping Players` :type "Array of Actor Object Reference"))
  (return (`self.GetOverlappingActors` self "/Game/Blueprints/Character/BP_MamaLava_Player.BP_MamaLava_Player_C")))

(fn `UserConstructionScript`
  (`parent.UserConstructionScript`))