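; Spline platform generator that builds a platform as a chain of spawned spline mesh segment actors along SplineCurve.
; GenerateCurve stores the mesh, forward axis and local transform, then destroys the previously tracked segments and spawns new ones.
; Each segment's mesh bends between neighboring spline points using their locations and tangents, with a modulo wrap at the last point.
; DestroyAfterDelay starts a one-shot timer and calls the parent version.
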(event Custom|Event%20Generate%20Curve
  (params (Platform_Mesh :type Static%20Mesh%20Object%20Reference) (Platform_Mesh_Forward_Axis :type ESplineMeshAxis%20Enum) (Platform_Mesh_Local_Transform :type Transform))
  (Variables|InputData|SetSplineMesh Platform_Mesh)
  (Variables|InputData|SetSplineMeshForwardAxis Platform_Mesh_Forward_Axis)
  (Variables|InputData|SetSplineMeshLocalTransform Platform_Mesh_Local_Transform)
  (Public|DestroyActorsinReferenceArray)
  (Public|CreateActorsinReferenceArray))

(event EventDestroyAfterDelay
  (Utilities|Time|SetTimerbyEvent (EventDispatchers|CreateEvent :!event DestroyActorsinReferenceArray) (Variables|Default|GetDestroyDelayInSeconds))
  (|CallParentFunction))

(fn ConstructionScript
  (|CallParentFunction)
  (Variables|InputData|SetSplineCurve 0))

(fn DestroyActorsinReferenceArray
  (for _array_element (Variables|OutputData|GetSplineMeshActorReferenceArray)
    (Actor|DestroyActor _array_element))
  (Utilities|Array|Clear (Variables|OutputData|GetSplineMeshActorReferenceArray))
  (return))

(fn CreateActorsinReferenceArray
  (for _index (range 0 (Utilities|GetNumberOfSplineMeshActorstoGenerate))
    (Utilities|FlowControl|Sequence
      (:then_0
        (bind _returnvalue (Game|SpawnActorfromClass "/Game/Blueprints/Environment/Spline/BP_Spline_Mesh_Platform_Segment_Actor_Base.BP_Spline_Mesh_Platform_Segment_Actor_Base_C" (Spline|GetTransformatSplinePoint (Variables|InputData|GetSplineCurve) (LocalVariables|GetCurrentPointIndex) "World" false) "Undefined" self 0))
        (bind _output_get (LocalVariables|SetCurrentSplineMeshActor _returnvalue))
        (Class|Actor|AddActorLocalTransform _output_get (Variables|InputData|GetSplineMeshLocalTransform) false false))
      (:then_1
        (bind _output_get_2 (LocalVariables|SetCurrentPointIndex _index))
        (LocalVariables|SetNextPointIndex (Math|Integer|%(Integer) (+ _output_get_2 1) (Spline|GetNumberOfSplinePoints (Variables|InputData|GetSplineCurve))))
        (Utilities|FlowControl|Sequence
          (:then_0
            (Components|StaticMesh|SetStaticMesh (Variables|/Script/Engine.SplineMeshActor|GetSplineMeshComponent (LocalVariables|GetCurrentSplineMeshActor)) (Variables|InputData|GetSplineMesh))
            (SplineMesh|SetForwardAxis (Variables|/Script/Engine.SplineMeshActor|GetSplineMeshComponent (LocalVariables|GetCurrentSplineMeshActor)) (Variables|InputData|GetSplineMeshForwardAxis) false))
          (:then_1
            (SplineMesh|SetStartandEnd (Variables|/Script/Engine.SplineMeshActor|GetSplineMeshComponent (LocalVariables|GetCurrentSplineMeshActor)) (Spline|GetLocationatSplinePoint (Variables|InputData|GetSplineCurve) (LocalVariables|GetCurrentPointIndex) "Local") (Spline|GetTangentatSplinePoint (Variables|InputData|GetSplineCurve) (LocalVariables|GetCurrentPointIndex) "Local") (Spline|GetLocationatSplinePoint (Variables|InputData|GetSplineCurve) (LocalVariables|GetNextPointIndex) "Local") (Spline|GetTangentatSplinePoint (Variables|InputData|GetSplineCurve) (LocalVariables|GetNextPointIndex) "Local") true :!class /Script/Engine.SplineMeshComponent))
          (:then_2)))))
  (return))