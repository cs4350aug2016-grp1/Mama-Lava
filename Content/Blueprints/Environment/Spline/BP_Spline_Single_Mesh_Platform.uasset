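; Spline-driven platform actor that builds a deformed single-mesh platform along its spline, optionally as a closed loop.
; The construction script rebuilds one spline mesh per segment, applying bank, width and thickness from a per-point struct array reset to defaults.
; ExtendSpline and RetractSpline add or remove end segments on open splines.
; Optional text renders number the points; boundary-mesh creation exists but is disconnected.
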(fn ConstructionScript
  (|CloseSplineifRequired)
  (Public|GenerateSplineMeshesfromSplineComponent))

(fn SetupSplineMeshComponent
  (params (Point_Index :type Integer) (Spline_Mesh_Component :type Spline%20Mesh%20Component%20Object%20Reference) (Platform_Segment_Mesh :type Static%20Mesh%20Object%20Reference) (Local_Location_Offset :type Vector) (Segment_Forward_Axis :type ESplineMeshAxis%20Enum) (Collision_Enabled_Type :type ECollisionEnabled%20Enum) (Is_Visible :type Boolean))
  (LocalVariables|SetCurrentLoopIndex Point_Index)
  (LocalVariables|SetCurrentSplineMeshComponent Spline_Mesh_Component)
  (LocalVariables|SetSplineMeshSegment Platform_Segment_Mesh)
  (LocalVariables|SetLocalMeshLocationOffset Local_Location_Offset)
  (LocalVariables|SetForwardAxis Segment_Forward_Axis)
  (LocalVariables|SetNextLoopIndex (Math|Integer|%(Integer) (+ (LocalVariables|GetCurrentLoopIndex) 1) (Variables|TrackData|GetNumSplinePoints)))
  (Utilities|FlowControl|Sequence
    (:then_0
      (Utilities|FlowControl|Sequence
        (:then_0
          (Utilities|FlowControl|Sequence
            (:then_0
              (LocalVariables|SetLocalStartLocation (.Location (Spline|GetLocationandTangentatSplinePoint (Variables|Default|GetSpline) (LocalVariables|GetCurrentLoopIndex) "Local")))
              (LocalVariables|SetLocalStartTangent (.Tangent (Spline|GetLocationandTangentatSplinePoint (Variables|Default|GetSpline) (LocalVariables|GetCurrentLoopIndex) "Local"))))
            (:then_1
              (LocalVariables|SetLocalEndLocation (.Location (Spline|GetLocationandTangentatSplinePoint (Variables|Default|GetSpline) (LocalVariables|GetNextLoopIndex) "Local")))
              (LocalVariables|SetLocalEndTangent (.Tangent (Spline|GetLocationandTangentatSplinePoint (Variables|Default|GetSpline) (LocalVariables|GetNextLoopIndex) "Local"))))))
        (:then_1
          (Utilities|FlowControl|Sequence
            (:then_0
              (LocalVariables|SetStartRoll (.platform_bank (Utilities|Array|Get(acopy) (Variables|TrackData|GetSplineDataStructArray) (LocalVariables|GetCurrentLoopIndex))))
              (LocalVariables|SetStartScale (Math|Vector2D|MakeVector2D (.platform_width (Utilities|Array|Get(acopy) (Variables|TrackData|GetSplineDataStructArray) (LocalVariables|GetCurrentLoopIndex))) (.platform_thickness (Utilities|Array|Get(acopy) (Variables|TrackData|GetSplineDataStructArray) (LocalVariables|GetCurrentLoopIndex))))))
            (:then_1
              (LocalVariables|SetEndRoll (.platform_bank (Utilities|Array|Get(acopy) (Variables|TrackData|GetSplineDataStructArray) (LocalVariables|GetNextLoopIndex))))
              (LocalVariables|SetEndScale (Math|Vector2D|MakeVector2D (.platform_width (Utilities|Array|Get(acopy) (Variables|TrackData|GetSplineDataStructArray) (LocalVariables|GetNextLoopIndex))) (.platform_thickness (Utilities|Array|Get(acopy) (Variables|TrackData|GetSplineDataStructArray) (LocalVariables|GetNextLoopIndex))))))))))
    (:then_1
      (Components|StaticMesh|SetStaticMesh (LocalVariables|GetCurrentSplineMeshComponent) (LocalVariables|GetSplineMeshSegment))
      (SplineMesh|SetForwardAxis (LocalVariables|GetCurrentSplineMeshComponent) (LocalVariables|GetForwardAxis) true)
      (Utilities|FlowControl|Sequence
        (:then_0
          (SplineMesh|SetStartandEnd (LocalVariables|GetCurrentSplineMeshComponent) (+ (LocalVariables|GetLocalStartLocation) (LocalVariables|GetLocalMeshLocationOffset)) (LocalVariables|GetLocalStartTangent) (+ (LocalVariables|GetLocalEndLocation) (LocalVariables|GetLocalMeshLocationOffset)) (LocalVariables|GetLocalEndTangent) true :!class /Script/Engine.SplineMeshComponent))
        (:then_1
          (Class|SplineMeshComponent|SetStartRoll (LocalVariables|GetCurrentSplineMeshComponent) (LocalVariables|GetStartRoll) true)
          (Class|SplineMeshComponent|SetEndRoll (LocalVariables|GetCurrentSplineMeshComponent) (LocalVariables|GetEndRoll) true))
        (:then_2
          (SplineMesh|SetStartScale (LocalVariables|GetCurrentSplineMeshComponent) (LocalVariables|GetStartScale) true :!class /Script/Engine.SplineMeshComponent)
          (SplineMesh|SetEndScale (LocalVariables|GetCurrentSplineMeshComponent) (LocalVariables|GetEndScale) true :!class /Script/Engine.SplineMeshComponent))))
    (:then_2
      (Collision|SetCollisionEnabled (LocalVariables|GetCurrentSplineMeshComponent) Collision_Enabled_Type)
      (Rendering|SetVisibility (LocalVariables|GetCurrentSplineMeshComponent) Is_Visible true)
      (Actor|SetOwner self))))

(fn GetSplineMeshComponent
  (params (Point_Index :type Integer))
  (return (.Spline_Mesh_Component (Utilities|Struct|BreakS_Spline_Single_Mesh_Platform_Single_Point_Data (Utilities|Array|Get(acopy) (Variables|TrackData|GetSplineDataStructArray) Point_Index)))))

(fn ExtendSpline
  (params (New_Spline_Point_World_Location :type Vector) (New_Mesh :type Static%20Mesh%20Object%20Reference) (New_Mesh_Local_Offset :type Vector) (New_Mesh_Forward_Axis :type ESplineMeshAxis%20Enum) (New_Mesh_Collision_Enabled_Type :type ECollisionEnabled%20Enum) (New_Mesh_Visibility :type Boolean))
  (if (not (Variables|TrackSetup|GetToLoop))
    (Spline|AddSplinePoint (Variables|Default|GetSpline) New_Spline_Point_World_Location "World")
    (Utilities|Array|Add (Variables|TrackData|GetSplineDataStructArray) (Variables|TrackData|GetDefaultSplineDataStruct))
    (Math|Integer|IncrementInt (Variables|TrackData|GetNumSplinePoints)
      (:%20%20
        (bind (_point_index _spline_mesh_component) (Private|CreateSplineMeshComponent (- (Utilities|Array|LastIndex (Variables|TrackData|GetSplineDataStructArray)) 1)))
        (Public|SetupSplineMeshComponent _point_index _spline_mesh_component New_Mesh New_Mesh_Local_Offset New_Mesh_Forward_Axis New_Mesh_Collision_Enabled_Type New_Mesh_Visibility))))
  (return))

(fn CreateSplineMeshComponent
  (params (Loop_Index :type Integer))
  (LocalVariables|SetLoopIndex Loop_Index)
  (bind _returnvalue (AddComponent|AddSplineMeshComponent false))
  (bind _structout (Utilities|Struct|SetmembersinS_Spline_Single_Mesh_Platform_Single_Point_Data (Utilities|Array|Get(acopy) (Variables|TrackData|GetSplineDataStructArray) (LocalVariables|GetLoopIndex)) _returnvalue))
  (Utilities|Array|SetArrayElem (Variables|TrackData|GetSplineDataStructArray) (LocalVariables|GetLoopIndex) _structout true)
  (return (LocalVariables|GetLoopIndex) _returnvalue))

(fn RetractSpline
  (bind _splinedatastructarray (Variables|TrackData|GetSplineDataStructArray))
  (bind _splinedatastructarray_2 (Variables|TrackData|GetSplineDataStructArray))
  (bind _splinedatastructarray_3 (Variables|TrackData|GetSplineDataStructArray))
  (if (not (Variables|TrackSetup|GetToLoop))
    (Components|DestroyComponent (.spline_mesh_component (Utilities|Array|Get(acopy) _splinedatastructarray (- (Utilities|Array|LastIndex _splinedatastructarray) 1))))
    (Utilities|Array|RemoveIndex _splinedatastructarray_2 (Utilities|Array|LastIndex _splinedatastructarray_2))
    (if (Variables|TrackSetup|GetToLoop)
      _
      (else
        (Utilities|Array|SetArrayElem _splinedatastructarray_3 (Utilities|Array|LastIndex _splinedatastructarray_3) (Variables|TrackData|GetDefaultSplineDataStruct))))
    (Spline|RemoveSplinePoint (Variables|Default|GetSpline) (- (Variables|TrackData|GetNumSplinePoints) 1))
    (Math|Integer|DecrementInt (Variables|TrackData|GetNumSplinePoints)
      (:%20%20
        _)))
  (return))

(fn CreateBoundarySplineMeshComponent
  (params (Loop_Index :type Integer))
  (LocalVariables|SetLoopIndex Loop_Index)
  (bind _returnvalue (AddComponent|AddSplineMeshComponent false))
  (bind _structout (Utilities|Struct|SetmembersinS_Spline_Single_Mesh_Platform_Single_Point_Data (Utilities|Array|Get(acopy) (Variables|TrackData|GetSplineDataStructArray) (LocalVariables|GetLoopIndex)) _returnvalue))
  (Utilities|Array|SetArrayElem (Variables|TrackData|GetSplineDataStructArray) (LocalVariables|GetLoopIndex) _structout true)
  (return (LocalVariables|GetLoopIndex) _returnvalue))

(fn GenerateSplineMeshesfromSplineComponent
  (Utilities|FlowControl|Sequence
    (:then_0
      (|StoreNumberofSplinePoints))
    (:then_1
      (|EliminatePreviouslyConstructedSplineMeshes))
    (:then_2
      (|PopulateArrayofSplineDataStructs))
    (:then_3
      (|ConstructPlatformBasedOnSpline))
    (:then_4
      (|DrawSplinePointNumbers))
    (:then_5
      (return))))

(fn GetLastSplineMeshComponentWidth
  (bind _spline_mesh_component (Public|GetSplineMeshComponent (- (Utilities|Array|LastIndex (Variables|TrackData|GetSplineDataStructArray)) 1)))
  (switch Utilities|FlowControl|Switch|SwitchonESplineMeshAxis (SplineMesh|GetForwardAxis _spline_mesh_component)
    (:X
      (return (.Y (Math|Vector|BreakVector (* (.BoxExtent (Collision|GetComponentBounds _spline_mesh_component)) 2.0)))))
    (:Y
      (return (.Y (Math|Vector|BreakVector (* (.BoxExtent (Collision|GetComponentBounds _spline_mesh_component)) 2.0)))))
    (:Z
      (return (.Y (Math|Vector|BreakVector (* (.BoxExtent (Collision|GetComponentBounds _spline_mesh_component)) 2.0)))))))