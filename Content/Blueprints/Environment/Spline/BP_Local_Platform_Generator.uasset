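; Local generator that builds platform segments along a supplied spline when GeneratePlatforms is called.
; It spawns actors of the given segment class at its root transform, passing TowerSegment to each.
; Each segment's spline mesh bends between neighbouring points using local-space positions and tangents, wrapping the next index.
; A lava-destruction cleanup exists but is unused, and creation never fills its reference array.
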(event Custom|Event%20Generate%20Platforms
  (params (Spline_Curve :type Spline%20Component%20Object%20Reference) (Segment_Class_To_Spawn :type Actor%20Class%20Reference) (NewParam :type Boolean))
  (Variables|InputData|SetSplineCurve Spline_Curve)
  (Variables|InputData|SetSegmentClassToSpawn Segment_Class_To_Spawn)
  (Public|CreateActorsinReferenceArray))

(fn ConstructionScript
  (|CallParentFunction))

(fn DestroyActorsinReferenceArray
  (for _array_element (Variables|OutputData|GetSplineMeshActorReferenceArray)
    (bind _asbp_platform_segment_base (Utilities|Casting|CastToBP_Platform_Segment_Base _array_element))
    (Default|LavaDestructionAfterDelay _asbp_platform_segment_base))
  (Utilities|Array|Clear (Variables|OutputData|GetSplineMeshActorReferenceArray))
  (return))

(fn CreateActorsinReferenceArray
  (for _index (range 0 (Utilities|GetNumberOfSplineMeshActorstoGenerate))
    (Utilities|FlowControl|Sequence
      (:then_0
        (bind _returnvalue (Game|SpawnActorfromClass (Variables|InputData|GetSegmentClassToSpawn) (Transformation|GetWorldTransform (Variables|Default|GetDefaultSceneRoot self)) "AlwaysSpawn" self 0))
        (bind _asbp_platform_segment_base (Utilities|Casting|CastToBP_Platform_Segment_Base _returnvalue)
          (:then
            (bind _output_get (LocalVariables|SetCurrentSplineMeshActor _asbp_platform_segment_base))
            (Variables|/Game/Blueprints/Environment/Spline/BP_Platform_Segment_Base.BP_Platform_Segment_Base_C|SetTowerSegment _output_get (Variables|InputData|GetTowerSegment)))
          (:CastFailed
            (return))))
      (:then_1
        (bind _output_get_2 (LocalVariables|SetCurrentPointIndex _index))
        (LocalVariables|SetNextPointIndex (Math|Integer|%(Integer) (+ _output_get_2 1) (Spline|GetNumberOfSplinePoints (Variables|InputData|GetSplineCurve))))
        (Utilities|FlowControl|Sequence
          (:then_0
            (SplineMesh|SetStartandEnd (Variables|/Script/Engine.SplineMeshActor|GetSplineMeshComponent (LocalVariables|GetCurrentSplineMeshActor)) (Spline|GetLocationatSplinePoint (Variables|InputData|GetSplineCurve) (LocalVariables|GetCurrentPointIndex) "Local") (Spline|GetTangentatSplinePoint (Variables|InputData|GetSplineCurve) (LocalVariables|GetCurrentPointIndex) "Local") (Spline|GetLocationatSplinePoint (Variables|InputData|GetSplineCurve) (LocalVariables|GetNextPointIndex) "Local") (Spline|GetTangentatSplinePoint (Variables|InputData|GetSplineCurve) (LocalVariables|GetNextPointIndex) "Local") true :!class /Script/Engine.SplineMeshComponent))))))
  (return))