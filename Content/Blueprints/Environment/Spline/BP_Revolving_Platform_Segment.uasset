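; Revolving platform segment that rotates around a pivot using its rotating movement component.
; On BeginPlay it picks the pivot from its spline mesh start X: a fixed point beyond a threshold, otherwise the XY location of the MamaLava game mode's platform generator.
; It then nudges itself up along local Z and applies that pivot as the movement's pivot translation.
; Construction is left to the parent class.
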(event `self.ReceiveBeginPlay`
  (bind _returnvalue_x (`KismetMathLibrary.BreakVector` (`SplineMeshComponent.GetStartPosition` (`self.SplineMeshComponent`))))
  (`|ExecutionSequence`
    (:`then_0`
      (bind _asbp_mama_lava_game_mode (cast `/Game/GameHandlers/BP_MamaLava_GameMode` (`GameplayStatics.GetGameMode`))))
    (:`then_1`
      (if (> _returnvalue_x 1000.0)
        (set `self.Pivot` (4500.0 0.0 0.0))
        (else
          (bind (_returnvalue_x_2 _returnvalue_y) (`KismetMathLibrary.BreakVector` (`self.K2_GetActorLocation` (`/Game/GameHandlers/BP_MamaLava_GameMode.PlatformGenerator` _asbp_mama_lava_game_mode))))
          (set `self.Pivot` (`KismetMathLibrary.MakeVector` _returnvalue_x_2 _returnvalue_y)))))
    (:`then_2`
      (`self.K2_AddActorLocalOffset` (0.0 0.0 40.0)))
    (:`then_3`
      (set `RotatingMovementComponent.PivotTranslation` (`self.Pivot`) (`self.RotatingMovement`)))))

(fn `UserConstructionScript`
  (`parent.UserConstructionScript`))