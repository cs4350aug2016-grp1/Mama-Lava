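; Tower generator actor that builds a tower layer by layer, keeping it ahead of the player as they gain height.
; BeginPlay calls GenerateLayer in a loop to lay down the initial stack.
; Each Tick compares TowerHeight with the player pawn's truncated Z and adds one layer whenever the gap falls below MinimumHeightAhead.
; GenerateLayer's implementation is not in these graphs, and the construction script is empty.
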(event `self.ReceiveBeginPlay`
  (for _ (range 11)
    (`self.GenerateLayer`)))

(event `self.ReceiveTick`
  (params (DeltaSeconds :type "Float (single-precision)"))
  (bind (_returnvalue_x _returnvalue_y _returnvalue_z) (`KismetMathLibrary.BreakVector` (`self.K2_GetActorLocation` (`GameplayStatics.GetPlayerPawn` 0))))
  (if (< (- (`self.TowerHeight`) (`KismetMathLibrary.FTrunc` _returnvalue_z)) (`self.MinimumHeightAhead`))
    (`self.GenerateLayer`)))

(fn `UserConstructionScript`)