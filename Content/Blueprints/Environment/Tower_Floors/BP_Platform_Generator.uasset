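; Tower-floor generator that spawns a ring of randomly spaced wooden platforms on BeginPlay.
; The construction script builds a regular-polygon spline from Radius and SideLength.
; Generate walks one spline length, picking random starts within MaximumJumpDistance and random ends, then spawns BP_Spline_Single_Mesh_Platform actors extended in SideLength steps.
; PreviousLayer stores platform distance ranges, seeding the next layer's start before old entries are removed.
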(event EventBeginPlay
  (CallFunction|Generate))

(event Collision|EventActorBeginOverlap
  (params (OtherActor :type Actor%20Object%20Reference)))

(event EventTick
  (params (DeltaSeconds :type Float%20%28single-precision%29)))

(fn ConstructionScript
  (|SetNumberOfSides)
  (|SetAngle)
  (|SetCenterToWallVector)
  (|InitializeSpline))

(fn Generate
  (|SetCurrent(Start)DistanceandEndDistance)
  (|Generateplatforms)
  (|Populateremainingspacewithplatforms)
  (for _index (range 0 (- (LocalVariables|GetNumberOfExistingPlatforms) 1))
    (Utilities|Array|RemoveIndex (Variables|Default|GetPreviousLayer))))

(fn CreatePlatform
  (params (Start :type Float%20%28single-precision%29) (End :type Float%20%28single-precision%29))
  (|SetAvailableRange Start End)
  (bind _splineplatformobject (|CreateSplinePlatformObject))
  (|GeneratePlatformUnits _splineplatformobject
    (:Completed
      (return (Utilities|Struct|MakeS_Platform_Data (LocalVariables|GetStartDistance) (LocalVariables|GetCurrentDistance))))))