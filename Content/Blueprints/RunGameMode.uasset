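; RunGameMode is a game mode that builds a tiled course with lava rising beneath it.
; On BeginPlay it spawns a lava actor at the origin and starts a looping timer that nudges it up one unit per tick.
; It also spawns a starting run of BaseTile_BP pieces, chained by feeding each tile's attach transform into the next spawn point.
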(event `self.ReceiveBeginPlay`
  (`self.AddLava`)
  (`KismetSystemLibrary.K2_SetTimer` null "RaiseLava" (`self.LavaRaiseRateInSecond`) true)
  (for _ (range 6)
    (`self.AddWallTile`)))

(fn `AddLava`
  (bind _returnvalue (`|SpawnActorFromClass` "/Game/Blueprints/Lava_BP.Lava_BP_C" (`KismetMathLibrary.MakeTransform` (0.0 0.0 0.0)) "Undefined" "OverrideRootScale"))
  (set `self.LavaRef` _returnvalue))

(fn `AddWallTile`
  (bind _returnvalue (`|SpawnActorFromClass` "/Game/Blueprints/BaseTile_BP.BaseTile_BP_C" (`self.NextSpawnPoint`) "Undefined" "OverrideRootScale"))
  (bind _attachtransform (`/Game/Blueprints/BaseTile_BP.GetAttachTransform` _returnvalue))
  (set `self.NextSpawnPoint` _attachtransform))

(fn `RaiseLava`
  (`self.K2_SetActorLocation` (`self.LavaRef`) (+ (`self.K2_GetActorLocation` (`self.LavaRef`)) (0.0 0.0 1.0)) false false))

(fn `UserConstructionScript`)