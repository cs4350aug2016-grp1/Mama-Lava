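; Maths function library with helpers for setting and reading single bits in a 32-bit integer.
; BitLeftShift emulates a left shift by doubling in a loop, returning zero for a full-width shift.
; SetBitAt and GetBitAt build their masks with it, then OR or AND them with the input.
; IsValidBitIndex guards both, so out-of-range indices leave bits unchanged or read as zero.
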(fn BitLeftShift
  (params (BitsIn :type Integer) (Shift :type Integer))
  (LocalVariables|SetBits BitsIn)
  (if (== Shift 32)
    (return 0)
    (else
      (for _index (range 1 Shift)
        (LocalVariables|SetBits (* (LocalVariables|GetBits) 2)))
      (return (LocalVariables|GetBits)))))

(fn SetBitat
  (params (BitsIn :type Integer) (Index :type Integer))
  (LocalVariables|SetBits BitsIn)
  (bind _isvalid (CallFunction|IsValidBitIndex Index))
  (if _isvalid
    (bind _bitsout (CallFunction|BitLeftShift 1 Index))
    (return (Class|KismetMathLibrary|OrIntInt _bitsout (LocalVariables|GetBits)))
    (else
      (return (LocalVariables|GetBits)))))

(fn GetBitat
  (params (BitsIn :type Integer) (Index :type Integer))
  (LocalVariables|SetBits BitsIn)
  (bind _isvalid (CallFunction|IsValidBitIndex Index))
  (if _isvalid
    (bind _bitsout (CallFunction|BitLeftShift 1 Index))
    (if (!= (Class|KismetMathLibrary|AndIntInt _bitsout (LocalVariables|GetBits)) 0)
      (return 1)
      (else
        (return 0)))
    (else
      (return 0))))

(fn IsValidBitIndex
  (params (Index :type Integer))
  (return (and (>= Index 0) (<= Index 31))))