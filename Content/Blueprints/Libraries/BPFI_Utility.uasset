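; Utility Blueprint in the Libraries folder with a function that generates a random emissive color.
; It randomly picks one of seven base colors: white or a slightly softened red, green, blue, yellow, magenta or cyan.
; Each RGB channel is then scaled by its own random factor to vary brightness and hue slightly, with alpha fixed at one.
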(fn GenerateRandomEmissiveColor
  (LocalVariables|SetRedMultiplier (Math|Random|RandomFloatinRange 0.75 1.0))
  (LocalVariables|SetGreenMultiplier (Math|Random|RandomFloatinRange 0.75 1.0))
  (LocalVariables|SetBlueMultiplier (Math|Random|RandomFloatinRange 0.75 1.0))
  (switch int (Math|Random|RandomIntegerinRange 0 6)
    (:Default
      _)
    (:0
      (LocalVariables|SetColor (Utilities|Struct|MakeLinearColor 1.0 1.0 1.0 1.0))
      (bind _output_get (LocalVariables|SetColor (Utilities|Struct|MakeLinearColor (* (.r (LocalVariables|GetColor)) (LocalVariables|GetRedMultiplier)) (* (.g (LocalVariables|GetColor)) (LocalVariables|GetGreenMultiplier)) (* (.b (LocalVariables|GetColor)) (LocalVariables|GetBlueMultiplier)) 1.0) :!label _label)))
    (:1
      (LocalVariables|SetColor (Utilities|Struct|MakeLinearColor 1.0 0.2 0.2 1.0))
      (goto _label))
    (:2
      (LocalVariables|SetColor (Utilities|Struct|MakeLinearColor 0.2 1.0 0.2 1.0))
      (goto _label))
    (:3
      (LocalVariables|SetColor (Utilities|Struct|MakeLinearColor 0.2 0.2 1.0 1.0))
      (goto _label))
    (:4
      (LocalVariables|SetColor (Utilities|Struct|MakeLinearColor 1.0 1.0 0.2 1.0))
      (goto _label))
    (:5
      (LocalVariables|SetColor (Utilities|Struct|MakeLinearColor 1.0 0.2 1.0 1.0))
      (goto _label))
    (:6
      (LocalVariables|SetColor (Utilities|Struct|MakeLinearColor 0.2 1.0 1.0 1.0))
      (goto _label)))
  (return _output_get))