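; Game mode for a tower climb above rising lava, spawning the platform generator, lava, starting wall segments and smoke roof.
; Each segment chains from the last's attach transform, sets a height-based saturating difficulty in GameState and triggers platform generation.
; StackWallSegment recycles free segments on top.
; After a delay, a timeline raises the lava with capped acceleration, catching up when the player gets too far ahead.
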(event `self.ReceiveBeginPlay`
  ;[1 1 1] Set character position to avoid blocking volume
  (`self.K2_SetActorLocation` (`GameplayStatics.GetPlayerCharacter` 0) (`KismetMathLibrary.MakeVector` (- (`self.TowerRadius`) 50.0) 0.0 25.0) false false)
  ;[1 1 1] Add platform generator
  (bind _returnvalue (`|SpawnActorFromClass` "/Game/Blueprints/Environment/Tower_Floors/BP_Platform_Generator.BP_Platform_Generator_C" (`self.NextSpawnPoint`) "Undefined" "OverrideRootScale" null (- (`self.TowerRadius`) 75.0) (`self.MaximumDifficultyLevel`)))
  (set `self.PlatformGenerator` _returnvalue)
  ;[1 1 1] Add lava
  (`self.AddLava`)
  (`KismetSystemLibrary.K2_SetTimerDelegate` (delegate `RaiseLava`) (`self.LavaStartDelay`))
  ;[1 1 1] Add walls
  (for _ (range (+ (`self.NumStartingSegments`) 1))
    (`self.AddWallTile`))
  ;[1 1 1] Add Tower Roof
  (`|SpawnActorFromClass` "/Game/Blueprints/Environment/Tower_Roof/BP_SmokeRoof.BP_SmokeRoof_C" (`self.NextSpawnPoint`) "Undefined" "OverrideRootScale"))

(event `RaiseLava`
  (bind (_returnvalue_x _returnvalue_y _returnvalue_z) (`KismetMathLibrary.BreakVector` (`self.K2_GetActorLocation` (`GameplayStatics.GetPlayerCharacter` 0))))
  (bind (_returnvalue_x_2 _returnvalue_y_2 _returnvalue_z_2) (`KismetMathLibrary.BreakVector` (`self.K2_GetActorLocation` (`self.LavaRef`))))
  ;[1 1 1] Add lava
  (bind (_direction _value) (`Timeline|Value`)
    (:`Update`
      (`self.K2_AddActorLocalOffset` (`self.LavaRef`) (`KismetMathLibrary.MakeVector` 0.0 0.0 (`KismetMathLibrary.Lerp` 0.0 (`KismetMathLibrary.FMax` (`KismetMathLibrary.FMax` (- (- _returnvalue_z _returnvalue_z_2) (`self.LavaMaxDistanceFromPawn`))) (`self.LavaRiseDistance`)) _value)) false false)
      (if (< (`self.LavaRiseDistance`) (`self.LavaMaxRiseDistance`))
        (set `self.LavaRiseDistance` (+ (`self.LavaRiseDistance`) (`self.LavaAccelerationRate`)))))))

(fn `Add Platform`
  (bind _platformgenerator (`self.PlatformGenerator`))
  (bind _nextspawnpoint_location (`KismetMathLibrary.BreakTransform` (`self.NextSpawnPoint`)))
  (`SceneComponent.K2_SetWorldLocation` (`/Game/Blueprints/Environment/Tower_Floors/BP_Platform_Generator.DefaultSceneRoot` _platformgenerator) _nextspawnpoint_location false false)
  (`/Game/Blueprints/Environment/Tower_Floors/BP_Platform_Generator.Generate` _platformgenerator))

(fn `AddLava`
  (bind _returnvalue (`|SpawnActorFromClass` "/Game/Blueprints/Environment/Lava/BP_Lava.BP_Lava_C" (`KismetMathLibrary.MakeTransform` (0.0 0.0 -200.0)) "Undefined" "OverrideRootScale" null (`self.TowerRadius`)))
  (set `self.LavaRef` _returnvalue))

(fn `AddWallTile`
  (bind _returnvalue (`|SpawnActorFromClass` "/Game/Blueprints/Environment/Tower_Wall/BP_Tower_Segment.BP_Tower_Segment_C" (`self.NextSpawnPoint`) "Undefined" "OverrideRootScale" null (`self.TowerRadius`) (`self.DefaultTowerSegmentHeight`) (- (`self.TowerRadius`) (`self.PlatformWidth`)) (`self.MaxNumberOfCoins`) (`self.PowerUpProbability`)))
  (`KismetArrayLibrary.Array_Add` (`self.TowerSegments`) _returnvalue)
  (bind _attachtransform (`/Game/Blueprints/Environment/Tower_Wall/BP_Tower_Segment.GetAttachTransform` _returnvalue))
  (set `self.NextSpawnPoint` _attachtransform)
  (`self.UpdateDifficultyLevel`)
  (set `/Game/Blueprints/Environment/Tower_Floors/BP_Platform_Generator.CurrentTowerSegment` _returnvalue (`self.PlatformGenerator`))
  (`self.Add Platform`))

(fn `StackWallSegment`
  (`KismetSystemLibrary.PrintString` "Stacking a free segment on top")
  (for _array_element (`self.TowerSegments`)
    (if (`/Game/Blueprints/Environment/Tower_Wall/BP_Tower_Segment.IsFree` _array_element)
      (`self.K2_SetActorTransform` _array_element (`self.NextSpawnPoint`) false false)
      (bind _attachtransform (`/Game/Blueprints/Environment/Tower_Wall/BP_Tower_Segment.GetAttachTransform` _array_element))
      (set `self.NextSpawnPoint` _attachtransform)
      (set `/Game/Blueprints/Environment/Tower_Wall/BP_Tower_Segment.IsFree` false _array_element)
      (`/Game/Blueprints/Environment/Tower_Wall/BP_Tower_Segment.ResetTrigger` _array_element))))

(fn `UpdateDifficultyLevel`
  (bind _nextspawnpoint (`self.NextSpawnPoint`))
  (bind _returnvalue (`KismetMathLibrary.Square` (.z (.location _nextspawnpoint))))
  (bind _asbp_mama_lava_game_state (cast `/Game/GameHandlers/BP_MamaLava_GameState` (`GameplayStatics.GetGameState`)))
  (set `/Game/GameHandlers/BP_MamaLava_GameState.CurrentDifficultyLevel` (+ 1 (`KismetMathLibrary.FTrunc` (/ (* (`self.MaximumDifficultyLevel`) _returnvalue) (+ _returnvalue (* (* (`self.GentlenessOfDifficultyRise`) 10000) (.z (.location _nextspawnpoint))))))) _asbp_mama_lava_game_state))

(fn `UserConstructionScript`)