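; Game mode for a climb-above-rising-lava game, driving tower stacking, lava rise and difficulty.
; Segment stacking delegates to TowerGenerator and starts the lava once after the first few segments.
; A timeline moves the lava by an accelerating, capped step, jumping further when the player gets too far ahead.
; Helpers pick random free reachable segments matching the difficulty level, which saturates toward a maximum as spawn height grows.
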(event Custom|StackTowerSegment
  (Default|StackSegment (Variables|Default|GetTowerGenerator))
  ;[1 1 1] Check auto start
  (if (<= (Variables|Default|GetStackCount) 4)
    (Math|Integer|IncrementInt (Variables|Default|GetStackCount))
    (else
      (Utilities|FlowControl|DoOnce false
        (:Completed
          (CallFunction|RaiseLava))))))

(event Custom|RaiseLava
  (Variables|/Game/Blueprints/Environment/Lava/BP_Lava.BP_Lava_C|SetIsRising (Variables|Lava|GetLava) true)
  (Default|PlayEruption (Variables|Lava|GetLava))
  (bind _data (Timeline|Timeline_0 Play)
    (:Update
      (Transformation|AddActorLocalOffset (Variables|Lava|GetLava) (Math|Vector|MakeVector 0.0 0.0 (Math|Float|Lerp 0.0 (Math|Float|Max(Float) (Math|Float|Max(Float) (- (- (.z (Transformation|GetActorLocation (Game|GetPlayerCharacter 0))) (.z (Transformation|GetActorLocation (Variables|Lava|GetLava)))) (Variables|Lava|GetLavaMaxDistanceFromPawn)) 0.0) (Variables|Lava|GetLavaRiseDistance)) _data)) false false)
      ;[1 1 1] Increases lava rise distance by constant increase if not already at max rise distance
      (if (< (Variables|Lava|GetLavaRiseDistance) (Variables|Lava|GetLavaMaxRiseDistance))
        (Variables|Lava|SetLavaRiseDistance (+ (Variables|Lava|GetLavaRiseDistance) (Variables|Lava|GetLavaAccelerationRate)))))))

(event Custom|StopRaiseLava
  (Variables|/Game/Blueprints/Environment/Lava/BP_Lava.BP_Lava_C|SetIsRising (Variables|Lava|GetLava) false)
  (bind _data (Timeline|Timeline_0 Stop)
    (:Update
      (Transformation|AddActorLocalOffset (Variables|Lava|GetLava) (Math|Vector|MakeVector 0.0 0.0 (Math|Float|Lerp 0.0 (Math|Float|Max(Float) (Math|Float|Max(Float) (- (- (.z (Transformation|GetActorLocation (Game|GetPlayerCharacter 0))) (.z (Transformation|GetActorLocation (Variables|Lava|GetLava)))) (Variables|Lava|GetLavaMaxDistanceFromPawn)) 0.0) (Variables|Lava|GetLavaRiseDistance)) _data)) false false)
      ;[1 1 1] Increases lava rise distance by constant increase if not already at max rise distance
      (if (< (Variables|Lava|GetLavaRiseDistance) (Variables|Lava|GetLavaMaxRiseDistance))
        (Variables|Lava|SetLavaRiseDistance (+ (Variables|Lava|GetLavaRiseDistance) (Variables|Lava|GetLavaAccelerationRate)))))))

(event EventBeginPlay)

(event EventTick
  (params (DeltaSeconds :type Float%20%28single-precision%29)))

(fn ConstructionScript)

(fn GetRandomFreeSegment
  (Development|PrintString "Hello")
  (Utilities|IsValid (Variables|Default|GetTopSegment)
    (:Is%20Valid
      (Utilities|Array|Clear (LocalVariables|GetFreeSegments))
      (Utilities|FlowControl|Sequence
        (:then_0
          ;[1 1 1] Get all the free segments that are reachable
          (for _array_element (Variables|/Game/Blueprints/Environment/Tower_Wall/BP_Tower_Segment.BP_Tower_Segment_C|GetReachableSegments (Variables|Default|GetTopSegment))
            (Utilities|IsValid _array_element
              (:Is%20Valid
                (if (and (Variables|/Game/Blueprints/Environment/Tower_Wall/BP_Tower_Segment.BP_Tower_Segment_C|GetIsFree _array_element) (== (Variables|/Game/Blueprints/Environment/Tower_Wall/BP_Tower_Segment.BP_Tower_Segment_C|GetDifficultyLevel _array_element) (Utilities|GetDifficultyLevel)))
                  (Utilities|Array|Add (LocalVariables|GetFreeSegments) _array_element))))))
        (:then_1
          ;[1 1 1] Pick randomly a free segment and return it
          (return (Utilities|Array|Get(acopy) (LocalVariables|GetFreeSegments) (Math|Random|RandomIntegerinRange 0 (- (Utilities|Array|Length (LocalVariables|GetFreeSegments)) 1)))))))
    (:Is%20Not%20Valid
      (return 0))))

(fn UpdateDifficultyLevel
  (bind _towergenerator (Variables|Default|GetTowerGenerator))
  (bind _nextspawnpoint (Variables|Default|GetNextSpawnPoint))
  (bind _returnvalue (Math|Float|Square (.z (.location _nextspawnpoint))))
  (bind _gentlenessdifficultrise (Variables|/Game/Blueprints/Environment/Tower_Wall/BP_TowerGenerator.BP_TowerGenerator_C|GetGentlenessDifficultRise _towergenerator))
  (bind _returnvalue_2 (* _gentlenessdifficultrise 1e+04))
  (bind _returnvalue_3 (* (.z (.location _nextspawnpoint)) _returnvalue_2))
  (bind _returnvalue_4 (+ _returnvalue _returnvalue_3))
  (bind _asbp_mama_lava_game_state (Utilities|Casting|CastToBP_MamaLava_GameState (Game|GetGameState)))
  ;[1 1 1] Handle division by 0
  (if (== _returnvalue_4 0.0)
    (Variables|/Game/GameHandlers/BP_MamaLava_GameState.BP_MamaLava_GameState_C|SetCurrentDifficultyLevel _asbp_mama_lava_game_state 1)
    (else
      (Variables|/Game/GameHandlers/BP_MamaLava_GameState.BP_MamaLava_GameState_C|SetCurrentDifficultyLevel _asbp_mama_lava_game_state (+ 1 (Math|Float|Truncate (/ (* (Variables|/Game/Blueprints/Environment/Tower_Wall/BP_TowerGenerator.BP_TowerGenerator_C|GetMaxDifficultyLevel (Variables|Default|GetTowerGenerator)) _returnvalue) _returnvalue_4)))))))