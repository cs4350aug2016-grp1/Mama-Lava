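; Game State Blueprint for MamaLava that currently holds only test scaffolding for runtime spline platform generation.
; GenerateTestSpline spawns a looping BP_Spline_Single_Mesh_Platform_Old with wooden platform meshes and stores it in TestGeneratedSpline.
; It then exercises that actor's API by extending, retracting and re-extending the spline through hardcoded points.
; BeginPlay and the construction script are empty, and the event graph's call to the test never runs.
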(event `self.ReceiveBeginPlay`)

(fn `UserConstructionScript`)